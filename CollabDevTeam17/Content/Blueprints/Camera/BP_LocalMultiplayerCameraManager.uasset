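; Player camera manager that sets up a single BP_LocalMultiplayerCamera for local multiplayer.
; The SetUpCamera event spawns and stores the camera only when none exists in the level.
; It then sets that camera as the owning player controller's view target.
; When a camera already exists, the event leaves the view target untouched.
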(event `SetUpCamera`
  ; Spawns camera when player exists
  (bind _outactors (`GameplayStatics.GetAllActorsOfClass` "/Game/Blueprints/Camera/BP_LocalMultiplayerCamera.BP_LocalMultiplayerCamera_C"))
  (if (`KismetArrayLibrary.Array_IsEmpty` _outactors)
    (bind _returnvalue (`|SpawnActorFromClass` "/Game/Blueprints/Camera/BP_LocalMultiplayerCamera.BP_LocalMultiplayerCamera_C" (`self.Spawn Transform`) "Undefined" "MultiplyWithRoot" null null))
    (set `self.Camera` _returnvalue)
    (`PlayerController.SetViewTargetWithBlend` (`self.GetOwningPlayerController`) (`self.Camera`) 0.0 "VTBlend_Linear" 0.0 false)))

(fn `UserConstructionScript`)