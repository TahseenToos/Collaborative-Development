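; Shared camera actor for local multiplayer that follows and frames all player pawns.
; BeginPlay waits a tick, then caches the player pawns and a BP_Midpoint anchor.
; Each Tick moves the actor to their averaged position at fixed height, with the anchor's weight multiplying only its X coordinate.
; The spring arm lengthens with the farthest player's distance from that point, using a clamped range remap to zoom out.
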(event `self.ReceiveBeginPlay`
  ; Finds all active players
  (`KismetSystemLibrary.DelayUntilNextTick`)
  (bind _returnvalue (`GameModeBase.GetNumPlayers` (`GameplayStatics.GetGameMode`)))
  (for _index (range _returnvalue)
    (bind _returnvalue_2 (`GameplayStatics.GetPlayerPawn` _index))
    (`/Engine/EditorBlueprintResources/StandardMacros.IsValid` _returnvalue_2
      (:`Is Valid`
        (`KismetArrayLibrary.Array_AddUnique` (`self.Players`) _returnvalue_2))))
  (bind _returnvalue_3 (`GameplayStatics.GetActorOfClass` "/Game/Blueprints/Gameplay/LevelActors/BP_Midpoint.BP_Midpoint_C"))
  (set `self.Midpoint` _returnvalue_3))

(event `self.ReceiveTick`
  (params (DeltaSeconds :type "Float (single-precision)"))
  (bind _midpoint (`self.Midpoint`))
  (bind (_returnvalue_x _returnvalue_y) (`KismetMathLibrary.BreakVector` (/ (`self.Player Midpoint`) (+ (`self.Midpoint Weighting`) (`KismetArrayLibrary.Array_Length` (`self.Players`))))))
  ; Resets values before recalculation
  (set `self.Player Midpoint` (0.0 0.0 0.0))
  ; Finds the midpoint between all players
  (for _array_element (`self.Players`)
    (set `self.Player Midpoint` (+ (`self.Player Midpoint`) (`self.K2_GetActorLocation` _array_element))))
  ; Allows camera view to grow when player moves out of camera range
  (`/Engine/EditorBlueprintResources/StandardMacros.IsValid` _midpoint
    (:`Is Valid`
      (set `self.Player Midpoint` (+ (`self.Player Midpoint`) (* (`self.K2_GetActorLocation` _midpoint) (`KismetMathLibrary.MakeVector` (`KismetMathLibrary.Conv_IntToDouble` (`self.Midpoint Weighting`)) 1.0 1.0)))))
    (:`Is Not Valid`
      _))
  (`self.K2_SetActorLocation` (`KismetMathLibrary.MakeVector` _returnvalue_x _returnvalue_y 40.0))
  (set `self.GreatestDistanceFromMidpoint` 0.0)
  (for _array_element_2 (`self.Players`)
    (bind _returnvalue (`KismetMathLibrary.Vector_Distance` (`self.K2_GetActorLocation` _array_element_2) (`self.K2_GetActorLocation`)))
    (if (< (`self.GreatestDistanceFromMidpoint`) _returnvalue)
      (set `self.GreatestDistanceFromMidpoint` _returnvalue)))
  (set `SpringArmComponent.TargetArmLength` (* (`KismetMathLibrary.MapRangeClamped` (`self.GreatestDistanceFromMidpoint`) (`self.Movement Range`) (`self.Max Movement Range`) 1.0 (`self.Max Movement Range Multiplier`)) (`self.Min Arm Length`)) (`self.SpringArm`)))

(fn `UserConstructionScript`)