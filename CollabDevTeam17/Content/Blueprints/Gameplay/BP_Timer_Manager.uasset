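; Timer manager Blueprint that runs an intro countdown when play begins, ahead of a gameplay countdown that is still an empty stub.
; A looping one-second timer is set by event, and the countdown logic decrements the remaining count, using debug prints as a placeholder for UI.
; At zero it calls the gameplay countdown event, prints a start message, resets the count and clears the timer by handle.
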(event `self.ReceiveBeginPlay`
  ; Starts the "Start Intro Countdown" timer.
  (`self.Start Intro Coundown`))

(event `Start Intro Coundown`
  ; Intro Countdown Timer, Set Timer.
  (set `self.Current Intro Countdown` (`self.Intro Countdown Length`))
  (bind _returnvalue (`KismetSystemLibrary.K2_SetTimerDelegate` (`|CreateDelegate` :!event `Start Countdown Timer`) 1.0 true))
  (set `self.Countdown Timer Handler` _returnvalue))

(event `Start Countdown Timer`
  (bind _current_intro_countdown (`self.Current Intro Countdown`))
  ; Starts the logic behind the timer.
  (if (> (`self.Current Intro Countdown`) 0.0)
    ; This is where you should change UI display
    (`KismetSystemLibrary.PrintString` (`KismetStringLibrary.Conv_DoubleToString` _current_intro_countdown))
    ; If Intro Countdown Timer is active, logic.
    (`/Engine/EditorBlueprintResources/StandardMacros.DecrementFloat` _current_intro_countdown)
    (else
      (`self.Start Gameplay Countdown`)
      (`KismetSystemLibrary.PrintString` "START!")
      ; If Intro Countdown Timer is not active, logic.
      (set `self.Current Intro Countdown` (`self.Intro Countdown Length`))
      (`KismetSystemLibrary.K2_ClearAndInvalidateTimerHandle` (`self.Countdown Timer Handler`)))))

(event `Start Gameplay Countdown`)