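; BP_AIFishActor is an AI fish character that trails an assigned actor in front of it, taking its skeletal mesh from fish info at construction.
; BeginPlay scales and rotates the mesh, caches the default walk speed and starts a fast looping timer.
; The follow event uses AIMoveTo toward a point behind the leader once the gap grows, switching to boosted speed when it falls further back.
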(event `self.ReceiveBeginPlay`
  (`KismetSystemLibrary.K2_SetTimerDelegate` (`|CreateDelegate` :!event `Follow Actor Infront`) 0.1 true)
  (set `self.Default Max Walk Speed` (`CharacterMovementComponent.MaxWalkSpeed` (`self.CharacterMovement`)))
  (`SceneComponent.SetRelativeScale3D` (`self.Mesh`) (0.15 0.15 0.15))
  (`SceneComponent.K2_SetRelativeRotation` (`self.Mesh`) (struct :`Pitch` 90.0 :`Yaw` -90.0) false false))

(event `Follow Actor Infront`
  (bind _actor_infront (`self.Actor Infront`))
  (bind _actor_infront_2 (`self.Actor Infront`))
  (bind _returnvalue (`KismetMathLibrary.Vector_Distance` (`self.K2_GetActorLocation` _actor_infront) (`self.K2_GetActorLocation`)))
  (`/Engine/EditorBlueprintResources/StandardMacros.IsValid` _actor_infront
    (:`Is Valid`
      (if (> _returnvalue 150.0)
        (if (> _returnvalue 200.0)
          (if (`self.Not Boosted`)
            (set `self.Not Boosted` false)
            (set `CharacterMovementComponent.MaxWalkSpeed` (`self.Boosted Max Walk Speed`) (`self.CharacterMovement`)))
          (else
            (set `self.Not Boosted` true)
            (set `CharacterMovementComponent.MaxWalkSpeed` (`self.Default Max Walk Speed`) (`self.CharacterMovement`))))
        (`|AIMoveTo` self (- (`self.K2_GetActorLocation` _actor_infront_2) (* (`KismetMathLibrary.Vector_Normal2D` (`self.GetActorForwardVector` _actor_infront_2)) 75.0)) null)))))

(fn `Set Mesh`
  (params (`Skeletal Mesh Asset` :type "SkeletalMesh Object Reference"))
  (set `SkeletalMeshComponent.SkeletalMeshAsset` `Skeletal Mesh Asset` (`self.Mesh`)))

(fn `Update Actor Infront`
  (params (`Actor Infront` :type "Actor Object Reference"))
  (set `self.Actor Infront` `Actor Infront`))

(fn `UserConstructionScript`
  (`self.Set Mesh` (`.FishMesh_5_85CAB8174A5AB92EE281ED823E21A737` (break `/Game/Blueprints/Gameplay/Structs/SCaughtFish` (`self.FIsh Info`)))))