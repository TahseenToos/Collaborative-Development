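; BP_Crown is a spinning crown pawn that travels to and attaches to a winning actor.
; A self-restarting Timeline continuously drives the yaw of its Cube.
; MoveToActor uses AIMoveTo toward the stored WinnerActor, then calls its AddCrown with itself whether the move succeeds or fails.
; LeavePlayer calls RemoveCrown on a valid winner, which is assigned and read through setter and getter functions.
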(event `self.ReceiveBeginPlay`
  (bind (_direction _newtrack_0) (`Timeline|Timeline` :!via `PlayFromStart` :!label _label)
    (:`Update`
      (`SceneComponent.K2_SetWorldRotation` (`self.Cube`) (`KismetMathLibrary.MakeRotator` 0.0 0.0 _newtrack_0) false false))
    (:`Finished`
      (goto _label :!via `PlayFromStart`))))

(event `Move To Actor`
  (bind _winneractor (`self.WinnerActor`))
  (`|AIMoveTo` self (0.0 0.0 0.0) _winneractor 1.0
    (:`OnSuccess`
      _)
    (:`OnFail`
      _))
  (`/Game/Blueprints/Gameplay/Character/BP_PlayerCharacter.Add Crown` _winneractor self))

(event `Leave Player`
  (bind _winneractor (`self.WinnerActor`))
  (`/Engine/EditorBlueprintResources/StandardMacros.IsValid` _winneractor
    (:`Is Valid`
      (`/Game/Blueprints/Gameplay/Character/BP_PlayerCharacter.Remove Crown` _winneractor))))

(fn `Get Winner Actor`
  (returns (`Winner Actor` :type "/Game/Blueprints/Gameplay/Character/BP_PlayerCharacter Object Reference"))
  (return (`self.WinnerActor`)))

(fn `Set Winner Actor`
  (params (WinnerActor :type "/Game/Blueprints/Gameplay/Character/BP_PlayerCharacter Object Reference"))
  (set `self.WinnerActor` WinnerActor))

(fn `UserConstructionScript`)