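; Game mode component that manages a pool of pre-placed sea mines, switching random ones on and off by toggling visibility and collision.
; Mines register into an inactive array; once the timer manager's countdown reaches half, a countdown enables random mines up to the current maximum.
; Deactivated mines return to the pool and start a respawn countdown.
; Later timer updates adjust the maximum from a time-keyed map and check for excess or missing mines.
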(event `OnRegisterMineLocation`
  (params (RegisteringMine :type "/Game/Blueprints/Gameplay/LevelActors/BP_SeaMine Object Reference"))
  ; Registers mines to an array to store their locations. Then hide them immediately.
  (`KismetArrayLibrary.Array_Add` (`self.InactiveMinesArray`) RegisteringMine)
  (set `self.AvailableMineCount` (`self.MaximumMineCount`)))

(event `IncreaseAvailableMines`
  (params (DeactivatedMine :type "/Game/Blueprints/Gameplay/LevelActors/BP_SeaMine Object Reference"))
  (bind _activeminesarray (`self.ActiveMinesArray`))
  ; Increases the maximum available mine count.
  ;; Removes the mine from the active mine array and adding it back to the inactive mine array.
  (`KismetArrayLibrary.Array_RemoveItem` _activeminesarray (`|GetArrayItem` _activeminesarray (`KismetArrayLibrary.Array_Find` _activeminesarray DeactivatedMine)))
  (`KismetArrayLibrary.Array_Add` (`self.InactiveMinesArray`) DeactivatedMine)
  ;; Increases the available mine count.
  (bind _output_get (set `self.AvailableMineCount` (+ (`self.AvailableMineCount`) 1)))
  ;; Checks if available and active mine count is less than maximum mine count.
  (if (not (<= (+ _output_get (`KismetArrayLibrary.Array_Length` (`self.ActiveMinesArray`))) (`self.MaximumMineCount`)))
    ;; If the count is over max mine count, removes all available mines.
    (set `self.AvailableMineCount` 0))
  ;; Checks if the respawn timer is active.
  (if (> (`self.AvailableMineCount`) 0)
    (if (not (`KismetSystemLibrary.K2_IsTimerActiveHandle` (`self.MineRespawnTimer`)))
      ;; Sets up the respawn timer, on the condition if it isn't already active.
      (set `self.CurrentRespawnCounter` (`self.MaxRespawnCounter`))
      (bind _returnvalue (`KismetSystemLibrary.K2_SetTimerDelegate` (`|CreateDelegate` :!event `OnMineRespawnTimerTrigger`) 1.0 true))
      (set `self.MineRespawnTimer` _returnvalue))))

(event `SetupInitalSpawn`
  (bind _timer_manager (`self.Timer Manager`))
  ; Sets up the inital spawning of mines.
  (set `self.CurrentRespawnCounter` (`self.MaxInitalSpawnCounter`))
  (`/Engine/EditorBlueprintResources/StandardMacros.IsValid` _timer_manager
    (:`Is Valid`
      (add `/Game/Blueprints/Gameplay/TimerAndGoal/BP_TimerManagerComponent.On Timer Update` _timer_manager (`|CreateDelegate` :!event `On Timer Update_Event`)))))

(event `OnMineRespawnTimerTrigger`
  ; Handles OnMineRespawnTimer. Simply iterates down until mines can spawn.
  (if (> (`self.CurrentRespawnCounter`) 0)
    (set `self.CurrentRespawnCounter` (- (`self.CurrentRespawnCounter`) 1))
    (else
      (`self.EnableRandomMine`)
      (`KismetSystemLibrary.K2_ClearAndInvalidateTimerHandle` (`self.MineRespawnTimer`)))))

(event `OnInitalSpawn`
  ; Handles the inital spawning of mines.
  (if (> (`self.CurrentRespawnCounter`) 0)
    (set `self.CurrentRespawnCounter` (- (`self.CurrentRespawnCounter`) 1))
    (else
      (`self.EnableRandomMine`)
      (`KismetSystemLibrary.K2_ClearAndInvalidateTimerHandle` (`self.InitalSpawnTimer`)))))

(event `EnableRandomMine`
  (bind _activeminesarray (`self.ActiveMinesArray`))
  ; Handles OnEnableMine
  ;; Checks if it's possible to spawn mines. Then enables the maximum amount of mines possible.
  (for _ (range (`self.AvailableMineCount`))
    (bind _output (`|GetArrayItem` (`self.InactiveMinesArray`) (stale `CreateRandomEnableIntegerHolder` _output_get)))
    ;; Validates if the chosen inactive mine is not already in the active mine array.
    (if (`KismetArrayLibrary.Array_IsValidIndex` _activeminesarray (`KismetArrayLibrary.Array_Find` _activeminesarray _output)) :!label _label
      ;; Gets a new random int, if the current random mine is already active.
      (`self.CreateRandomEnableIntegerHolder`)
      (goto _label)
      (else
        ;; Adding the mine to the active mine array, while also removing it from the inactive mine array.
        (`Actor.SetActorHiddenInGame` _output false)
        (`Actor.SetActorEnableCollision` _output true)
        (`KismetArrayLibrary.Array_Add` (`self.ActiveMinesArray`) _output)
        (`KismetArrayLibrary.Array_RemoveItem` (`self.InactiveMinesArray`) _output))))
  ;; Sets the mine count to zero after mines are spawned in.
  (set `self.AvailableMineCount` 0))

(event `self.ReceiveEndPlay`
  (params (EndPlayReason :type "EEndPlayReason Enum" :default "Destroyed"))
  (bind _activeminesarray (`self.ActiveMinesArray`))
  ; Handles OnEndPlay.
  ;; Removes all active mines and sets them to inactive.
  (for _array_element _activeminesarray
    (`Actor.SetActorHiddenInGame` _array_element true)
    (`Actor.SetActorEnableCollision` _array_element false)
    (`KismetArrayLibrary.Array_RemoveItem` _activeminesarray _array_element)
    (`KismetArrayLibrary.Array_Add` (`self.InactiveMinesArray`) _array_element))
  (set `self.AvailableMineCount` 0))

(event `CreateRandomEnableIntegerHolder`
  ; Handles OnEnableMine
  ;; Gets a random integer. Used in activating a random mine.
  (bind _output_get (set `self.EnableIntegerHolder` (`KismetMathLibrary.RandomInteger` (- (`KismetArrayLibrary.Array_Length` (`self.InactiveMinesArray`)) 1)))))

(event `RemoveRandomMine`
  (set `self.OverMaximumMineCount` (- (+ (`self.AvailableMineCount`) (`KismetArrayLibrary.Array_Length` (`self.ActiveMinesArray`))) (`self.MaximumMineCount`)))
  (for _ (range 1)
    (bind _output (`|GetArrayItem` (`self.ActiveMinesArray`) (stale `CreateRandomDisableIntegerHolder` _output_get)))
    (`Actor.SetActorHiddenInGame` _output true)
    (`Actor.SetActorEnableCollision` _output false)
    (`KismetArrayLibrary.Array_Add` (`self.InactiveMinesArray`))
    (`KismetArrayLibrary.Array_RemoveItem` (`self.ActiveMinesArray`)))
  (set `self.OverMaximumMineCount` 0))

(event `On Timer Update_Event`
  (params (`Remaining Time` :type Integer))
  (bind (_timer_manager_struct_startcountdownlength _timer_manager_struct_gameplaycountdownlength) (break `/Game/Blueprints/Gameplay/Structs/TimerManagerStruct/S_Timer_Manager_Structure` (`/Game/Blueprints/Gameplay/TimerAndGoal/BP_TimerManagerComponent.Timer Manager Struct` (`self.Timer Manager`))))
  ; Handles OnTimerUpdate_Event
  ;; Checks if mines are activated.
  (if (`self.bNotBeenActivated`)
    (if (<= (/ `Remaining Time` _timer_manager_struct_gameplaycountdownlength) 0.5)
      ;; Activates the mines.
      (bind _returnvalue (`KismetSystemLibrary.K2_SetTimerDelegate` (`|CreateDelegate` :!event `OnInitalSpawn`) 1.0 true))
      (set `self.InitalSpawnTimer` _returnvalue)
      (set `self.bNotBeenActivated` false))
    (else
      ;; Checks if the mine limit needs altering.
      (bind _result (`/Engine/EditorBlueprintResources/StandardMacros.IncrementInt` (`self.SecondsAfterActivation`))
        (:`  `
          (bind (_value _returnvalue_2) (`BlueprintMapLibrary.Map_Find` (`self.TimeVariableMaxActiveMines`) _result))
          (if _returnvalue_2
            ;; Comment
            (bind _output_get (set `self.MaximumMineCount` _value))
            (set `self.AvailableMineCount` (- _output_get (`KismetArrayLibrary.Array_Length` (`self.ActiveMinesArray`))))
            (set `self.ActivatedSecondsHolder` (`self.SecondsAfterActivation`))
            (`self.CheckMineCount`)
            (else
              ;; Checks for the mine count.
              (`self.CheckMineCount`)
              (`KismetSystemLibrary.PrintString` "Mine count check called"))))))))

(event `CreateRandomDisableIntegerHolder`
  (bind _output_get (set `self.DisableIntegerHolder` (`KismetMathLibrary.RandomInteger` (- (`KismetArrayLibrary.Array_Length` (`self.ActiveMinesArray`)) 1)))))

(event `CheckMineCount`
  ; Checks the mine count for if it's got too many or too few active/available mines.
  ;; Removes mines if there's too many mines.
  (if (and (> (+ (`self.AvailableMineCount`) (`KismetArrayLibrary.Array_Length` (`self.ActiveMinesArray`))) (`self.MaximumMineCount`)) (`self.bRemoveExtraMines`))
    (`self.RemoveRandomMine`)
    (`KismetSystemLibrary.PrintString` "Removing mines")
    (else
      ;; Enables mines if there's too few mines.
      (if (and (<= (`KismetArrayLibrary.Array_Length` (`self.ActiveMinesArray`)) 0) (< (`self.AvailableMineCount`) 0))
        (set `self.AvailableMineCount` (`self.MaximumMineCount`))
        (`self.EnableRandomMine`)
        (`KismetSystemLibrary.PrintString` "Adding mines")))))

(fn `Set Timer Manager`
  (params (`Timer Manager` :type "/Game/Blueprints/Gameplay/TimerAndGoal/BP_TimerManagerComponent Object Reference"))
  (set `self.Timer Manager` `Timer Manager`)
  (`self.SetupInitalSpawn`))