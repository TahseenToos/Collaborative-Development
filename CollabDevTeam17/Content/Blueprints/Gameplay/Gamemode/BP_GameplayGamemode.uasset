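; Gameplay game mode for a local four-player boat fishing game, handling player spawning, colours and round-end results.
; BeginPlay links the timer, goal and fishing spot managers, creates four local controllers, then spawns players from GameInstance input devices or a debug count.
; Spawned players receive numbered slots, boat colours and HUD score widgets.
; The start timer starts the game; SetLeaderboardWidget displays the leaderboard and saves scores to the GameInstance by input device.
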(event `self.ReceiveBeginPlay`
  (bind _bp_timermanagercomponent (`self.BP_TimerManagerComponent`))
  (bind _asbp_game_instance (cast `/Game/Blueprints/Gameplay/BP_GameInstance` (`GameplayStatics.GetGameInstance`)))
  (set `self.As BP Game Instance` _asbp_game_instance)
  (`/Game/Blueprints/Gameplay/TimerAndGoal/BP_TimerManagerComponent.Goal Manager Setter` _bp_timermanagercomponent (`self.BP_GoalManagerComponent`))
  (add `/Game/Blueprints/Gameplay/TimerAndGoal/BP_TimerManagerComponent.On Game Timer Finished` _bp_timermanagercomponent (`|CreateDelegate` :!event `Set Leaderboard Widget`))
  (`/Game/Blueprints/Gameplay/Gamemode/BP_FishingSpotManagerComponent.Gamemode Setter` (`self.BPC_FishingSpotManager`) self)
  (while (<= (`GameplayStatics.GetNumLocalPlayerControllers`) 3)
    ;[0.03101 0.06094 1 0.5] Makes sure there is a total of 4 player controllers in the level with the right mapping context
    (bind _returnvalue (`GameplayStatics.CreatePlayer` -1))
    (`KismetSystemLibrary.Delay` 0.01)
    (bind _returnvalue_2 (pcsubsystem `EnhancedInputLocalPlayerSubsystem` _returnvalue))
    (`/Engine/EditorBlueprintResources/StandardMacros.IsValid` _returnvalue_2
      (:`Is Valid`
        (`EnhancedInputSubsystemInterface.AddMappingContext` _returnvalue_2 "/Game/Inputs/Lobby/IMC_Pre-Join.IMC_Pre-Join" 0 (struct)))))
  ;[0 1 0.4763 0.5] Sets the default pawn from empty to the correct actor
  (set `self.DefaultPawnClass` (`self.Default Pawn Class`))
  (if (not (`self.Is Debugging?`))
    (bind _values (`BlueprintMapLibrary.Map_Values` (`/Game/Blueprints/Gameplay/BP_GameInstance.Player Numbers` (`self.As BP Game Instance`))))
    (for _array_element _values
      (bind _returnvalue_3 (`InputDeviceLibrary.GetPlayerControllerFromInputDevice` _array_element))
      (`self.Call Restart Player` _returnvalue_3))
    (else
      (for _index (range (+ (`self.Num of players -1`) 1))
        (`self.Call Restart Player` (`GameplayStatics.GetPlayerControllerFromID` _index))))))

(event `self.BP_TimerManagerComponent.On Start Timer Finished`
  (`self.On Start Game`))

(event `Set Leaderboard Widget`
  (bind _returnvalue (`GameplayStatics.GetPlayerControllerFromID` 0))
  (`WidgetBlueprintLibrary.SetInputMode_UIOnlyEx` _returnvalue null)
  (set `PlayerController.bShowMouseCursor` true _returnvalue)
  (bind _player_order (`/Game/UI/UI_HUD/WBP_HUD.Get Player Order` (`/Game/Blueprints/Gameplay/Gamemode/BP_GameplayUIManagerComponent.Screen HUD` (`self.BP_GameplayUIManagerComponent`))))
  (`WidgetLayoutLibrary.RemoveAllWidgets`)
  (bind _returnvalue_2 (`|CreateWidget` "/Game/UI/UI_HUD/WBP_RoundEndLeaderboard.WBP_RoundEndLeaderboard_C" null _player_order (`self.Players and Score`)))
  (`UserWidget.AddToViewport` _returnvalue_2 0)
  (for _array_element _player_order
    (bind _returnvalue_3 (`InputDeviceLibrary.GetPrimaryInputDeviceForUser` (`Pawn.GetPlatformUserId` _array_element)))
    (`/Game/Blueprints/Gameplay/BP_GameInstance.Save Player Score` (`self.As BP Game Instance`) _returnvalue_3 (`BlueprintMapLibrary.Map_Find` (`/Game/Blueprints/Gameplay/TimerAndGoal/BP_GoalManagerComponent.Player Map` (`self.BP_GoalManagerComponent`)) _array_element))))

(fn `Assigning player colours`
  (params (Selection :type Integer) (`Player Pawn` :type "/Game/Blueprints/Gameplay/Character/BP_PlayerCharacter Object Reference"))
  (bind _player_pawn (`local.Player Pawn`))
  (bind _player_pawn_2 (`local.Player Pawn`))
  (bind _player_pawn_3 (`local.Player Pawn`))
  (bind _player_pawn_4 (`local.Player Pawn`))
  ; Assigns player a colour
  (`|ExecutionSequence`
    (:`then_0`
      (switch `int` Selection
        (:`1`
          (set `/Game/Blueprints/Gameplay/Character/BP_PlayerCharacter.PlayerColour` (struct :`R` 1.0 :`A` 1.0) _player_pawn_3)
          (set `/Game/Blueprints/Gameplay/Character/BP_PlayerCharacter.Player Colour Text` "Red" _player_pawn_3))
        (:`2`
          (set `/Game/Blueprints/Gameplay/Character/BP_PlayerCharacter.PlayerColour` (struct :`R` 0.002831 :`B` 1.0 :`A` 1.0) _player_pawn_4)
          (set `/Game/Blueprints/Gameplay/Character/BP_PlayerCharacter.Player Colour Text` "Blue" _player_pawn_4))
        (:`3`
          (set `/Game/Blueprints/Gameplay/Character/BP_PlayerCharacter.PlayerColour` (struct :`R` 1.0 :`G` 0.842597 :`B` 0.001543 :`A` 1.0) _player_pawn_2)
          (set `/Game/Blueprints/Gameplay/Character/BP_PlayerCharacter.Player Colour Text` "Yellow" _player_pawn_2))
        (:`4`
          (set `/Game/Blueprints/Gameplay/Character/BP_PlayerCharacter.PlayerColour` (struct :`R` 0.009698 :`G` 1.0 :`A` 1.0) _player_pawn)
          (set `/Game/Blueprints/Gameplay/Character/BP_PlayerCharacter.Player Colour Text` "Green" _player_pawn))))
    (:`then_1`
      (`/Game/Blueprints/Gameplay/Character/BP_PlayerCharacter.Set Boat Colour` `Player Pawn`))))

(fn `Call Restart Player`
  (params (NewPlayer :type "Controller Object Reference"))
  (locals (`Player Pawn` :type "/Game/Blueprints/Gameplay/Character/BP_PlayerCharacter Object Reference"))
  (bind _returnvalue (`Controller.K2_GetPawn` NewPlayer))
  (bind _players (`self.Players`))
  (bind _player_num (`self.Player Num`))
  (`self.RestartPlayer` NewPlayer)
  (set `local.Player Pawn` null)
  (if (== (`self.Default Pawn Class`) (`GameplayStatics.GetObjectClass` _returnvalue))
    (bind _asbp_player_character (cast `/Game/Blueprints/Gameplay/Character/BP_PlayerCharacter` _returnvalue))
    (set `local.Player Pawn` _asbp_player_character)
    (if (not (> (`self.Player Num`) 4))
      (`self.Assigning player colours` (`self.Player Num`) (`local.Player Pawn`))
      ; Increments player number, ready for next player
      (`BlueprintMapLibrary.Map_Add` (`self.Players`) (`self.Player Num`) (`local.Player Pawn`))
      (`/Game/UI/UI_HUD/WBP_HUD.Set Up Player Score Widgets` (`/Game/Blueprints/Gameplay/Gamemode/BP_GameplayUIManagerComponent.Screen HUD` (`self.BP_GameplayUIManagerComponent`)) _player_num)
      (`/Engine/EditorBlueprintResources/StandardMacros.IncrementInt` _player_num
        (:`  `
          (return)))
      (else
        ; If Player joining is greater than the 4th, checks if player slots are missing, if there is, assigns the player
        (if (< (`BlueprintMapLibrary.Map_Length` _players) 4)
          (bind _keys (`BlueprintMapLibrary.Map_Keys` _players))
          (for _array_element _keys
            (for _index (range 1 5)
              (if (== _index _array_element)
                (`BlueprintMapLibrary.Map_Add` (`self.Players`) (`self.Player Num`) (`local.Player Pawn`))
                (`self.Assigning player colours` (`self.Player Num`) (`local.Player Pawn`))
                (set `self.Num Of Active Players` 5))))
          (`KismetSystemLibrary.PrintText` "Failed to assign player a number")
          (`KismetSystemLibrary.LogString` "FAILED to assign player a number (BP_GameplayGamemode)"))))))

(fn `Update Player Score`
  (params (Player :type "/Game/Blueprints/Gameplay/Character/BP_PlayerCharacter Object Reference (by ref)") (Points :type "Integer (by ref)"))
  (`BlueprintMapLibrary.Map_Add` (`self.Players and Score`) Player Points))

(fn `UserConstructionScript`)