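; Gamemode manager component that controls which fishing spots in the level are active during the game.
; On BeginPlay it binds to the gamemode's start event, gathers every BP_FishingSpot and registers itself as their manager.
; It activates a set number of random spots, sends deactivation warnings to active ones, and can swap one spot for a random pick.
; Two looping timers share one interval, the second set up shortly before the first interval ends.
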(event `self.ReceiveBeginPlay`
  ; Gets reference to all fishing spots in the level
  (`KismetSystemLibrary.DelayUntilNextTick`)
  (add `/Game/Blueprints/Gameplay/Gamemode/BP_GameplayGamemode.On Start Game` (`self.Gamemode`) (`|CreateDelegate` :!event `Set Up Fishing Spot Timer`))
  (bind _outactors (`GameplayStatics.GetAllActorsOfClass` (`self.Actor Class`)))
  (for _array_element _outactors
    (bind _asbp_fishing_spot (cast `/Game/Blueprints/Gameplay/LevelActors/BP_FishingSpot` _array_element))
    (`KismetArrayLibrary.Array_AddUnique` (`self.Fishing Spots`) _asbp_fishing_spot))
  (for _array_element_2 (`self.Fishing Spots`)
    (set `/Game/Blueprints/Gameplay/LevelActors/BP_FishingSpot.Manager` self _array_element_2)))

(event `Activate Fishing spots`
  ; Takes int in and activates that number of fishing spots
  (for _array_element (`self.Active Fishing Spots`)
    (`KismetArrayLibrary.Array_AddUnique` (`self.Fishing Spots`) _array_element)
    (`KismetArrayLibrary.Array_RemoveItem` (`self.Active Fishing Spots`) _array_element))
  (`KismetArrayLibrary.Array_Clear` (`self.Active Fishing Spots`))
  (while (> (`self.Fishing Spots to Activate`) (`KismetArrayLibrary.Array_Length` (`self.Active Fishing Spots`)))
    (`KismetArrayLibrary.Array_AddUnique` (`self.Active Fishing Spots`) (`KismetArrayLibrary.Array_Random` (`self.Fishing Spots`))))
  (for _array_element_2 (`self.Active Fishing Spots`)
    (`/Game/Blueprints/Gameplay/LevelActors/BP_FishingSpot.Activate Fishing Spot` _array_element_2)))

(event `Deactivate Fishing spots`
  ; Deactivates all active fishing spots
  (for _array_element (`self.Active Fishing Spots`)
    (`/Game/Blueprints/Gameplay/LevelActors/BP_FishingSpot.Deactivation Warning` _array_element)))

(event `Swap Fishing Spots`
  (params (`Fishing Spot` :type "/Game/Blueprints/Gameplay/LevelActors/BP_FishingSpot Object Reference"))
  (bind _active_fishing_spots (`self.Active Fishing Spots`))
  (bind _output_get (set `self.Fishing  Spot To Activate` (`KismetArrayLibrary.Array_Random` (`self.Fishing Spots`))))
  (`/Game/Blueprints/Gameplay/LevelActors/BP_FishingSpot.Activate Fishing Spot` _output_get)
  (`KismetArrayLibrary.Array_AddUnique` _active_fishing_spots _output_get)
  (`/Game/Blueprints/Gameplay/LevelActors/BP_FishingSpot.Deactivate Fishing Spot` `Fishing Spot`)
  (`KismetArrayLibrary.Array_RemoveItem` _active_fishing_spots `Fishing Spot`)
  (set `self.Fishing  Spot To Activate` null))

(event `Set Up Fishing Spot Timer`
  (bind _fishing_spot_intervals (`self.Fishing Spot Intervals`))
  (bind _fishing_spot_intervals_2 (`self.Fishing Spot Intervals`))
  (`KismetSystemLibrary.K2_SetTimerDelegate` (`|CreateDelegate` :!event `Activate Fishing spots`) _fishing_spot_intervals_2 true false (* _fishing_spot_intervals_2 -1.0))
  (`KismetSystemLibrary.Delay` (- (`self.Fishing Spot Intervals`) 2.61))
  (`KismetSystemLibrary.K2_SetTimerDelegate` (`|CreateDelegate` :!event `Deactivate Fishing spots`) _fishing_spot_intervals true false (* _fishing_spot_intervals -1.0)))

(fn `Gamemode Setter`
  (params (Gamemode :type "/Game/Blueprints/Gameplay/Gamemode/BP_GameplayGamemode Object Reference"))
  (set `self.Gamemode` Gamemode))