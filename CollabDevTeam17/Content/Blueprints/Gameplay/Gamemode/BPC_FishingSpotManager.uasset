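; Game mode component that manages which fishing spots in the level are active.
; On BeginPlay it caches the level's fishing spot actors with GetAllActorsOfClass.
; ActivateFishingspots draws random spots with AddUnique until the active list reaches the requested count, with no guard for requests exceeding available spots, then activates each.
; DeactivateFishingspots deactivates every active spot and clears the list.
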(event `self.ReceiveBeginPlay`
  ; Gets reference to all fishing spots in the level
  (bind _outactors (`GameplayStatics.GetAllActorsOfClass` (`self.Actor Class`)))
  (set `self.Fishing Spots` _outactors))

(event `Activate Fishing spots`
  (params (`Fishing Spots To Activate` :type Integer))
  ; Takes int in and activates that number of fishing spots
  (while (> `Fishing Spots To Activate` (`KismetArrayLibrary.Array_Length` (`self.Active Fishing Spots`)))
    (bind _asbp_fishing_spot (cast `/Game/Blueprints/Gameplay/BP_FishingSpot` (`KismetArrayLibrary.Array_Random` (`self.Fishing Spots`))))
    (`KismetArrayLibrary.Array_AddUnique` (`self.Active Fishing Spots`) _asbp_fishing_spot))
  (for _array_element (`self.Active Fishing Spots`)
    (`/Game/Blueprints/Gameplay/BP_FishingSpot.Activate Fishing Spot` _array_element)))

(event `Deactivate Fishing spots`
  ; Deactivates all active fishing spots
  (for _array_element (`self.Active Fishing Spots`)
    (`/Game/Blueprints/Gameplay/BP_FishingSpot.Deactivate Fishing Spot` _array_element))
  (`KismetArrayLibrary.Array_Clear` (`self.Active Fishing Spots`)))