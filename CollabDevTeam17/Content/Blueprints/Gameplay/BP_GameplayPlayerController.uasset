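; Player controller for local multiplayer gameplay that handles joining and input setup.
; It starts with a pre-join input context, and the join action asks the game mode to spawn a pawn if none is controlled.
; On possess, local controllers swap to the movement context after a short delay, and the local multiplayer camera manager sets up the camera.
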(event `self.ReceiveBeginPlay`
  (bind _returnvalue (subsystem `EnhancedInputLocalPlayerSubsystem`))
  ; Sets up join mapping
  (`KismetSystemLibrary.Delay` 0.1)
  (`/Engine/EditorBlueprintResources/StandardMacros.IsValid` _returnvalue
    (:`Is Valid`
      (`EnhancedInputSubsystemInterface.AddMappingContext` _returnvalue "/Game/Inputs/PlayerMovement/IMC_Pre-Join.IMC_Pre-Join" 0 (struct)))))

(event `self.ReceivePossess`
  (params (PossessedPawn :type "Pawn Object Reference"))
  ; Sorts mapping context and camera (if camera is not already sorted)
  (`|ExecutionSequence`
    (:`then_0`
      (if (`self.IsLocalPlayerController`)
        (`EnhancedInputSubsystemInterface.AddMappingContext` (subsystem `EnhancedInputLocalPlayerSubsystem`) "/Game/Inputs/PlayerMovement/IMC_PlayerMovement.IMC_PlayerMovement" 0 (struct))
        (`KismetSystemLibrary.Delay` 0.2)
        (message `EnhancedInputSubsystemInterface.RemoveMappingContext` (subsystem `EnhancedInputLocalPlayerSubsystem`) "/Game/Inputs/PlayerMovement/IMC_Pre-Join.IMC_Pre-Join" (struct))))
    (:`then_1`
      (bind _asbp_local_multiplayer_camera_manager (cast `/Game/Blueprints/Camera/BP_LocalMultiplayerCameraManager` (`self.PlayerCameraManager`)))
      (`/Game/Blueprints/Camera/BP_LocalMultiplayerCameraManager.SetUpCamera` _asbp_local_multiplayer_camera_manager))))

(event `EnhancedInput|/Game/Inputs/PlayerMovement/Keybinds/IA_JoinGame`
  (params (ActionValue :type Boolean) (ElapsedSeconds :type "Float (double-precision)") (TriggeredSeconds :type "Float (double-precision)") (InputAction :type "InputAction Object Reference" :default "/Game/Inputs/PlayerMovement/Keybinds/IA_JoinGame.IA_JoinGame"))
  ; Allows the player to join, if not already joined
  (:`Started`
    (`/Engine/EditorBlueprintResources/StandardMacros.IsValid` (`self.K2_GetPawn`)
      (:`Is Not Valid`
        (`GameModeBase.RestartPlayer` (`GameplayStatics.GetGameMode`) self)))))

(fn `UserConstructionScript`)