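; Gameplay game mode that matches the number of local players to the connected input devices for local multiplayer.
; BeginPlay sets a timer by event, and ControllerInputSetup compares the device count to the local player controller count.
; It loops, creating players or removing the last one along with its pawn until the counts match.
; The target count adds one when the project skips assigning a gamepad to player 1.
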(event `self.ReceiveBeginPlay`
  (`KismetSystemLibrary.K2_SetTimerDelegate` (`|CreateDelegate` :!event `ControllerInputSetup`)))

(event `ControllerInputSetup`
  (bind _returnvalue (`GameplayStatics.GetNumLocalPlayerControllers`))
  (bind (_outinputdevices _returnvalue_2) (`InputDeviceLibrary.GetAllConnectedInputDevices` :!label _label))
  (bind _returnvalue_3 (`KismetMathLibrary.Max` (select `bool` (`GameMapsSettings.GetSkipAssigningGamepadToPlayer1` (`GameMapsSettings.GetGameMapsSettings`)) :`false` _returnvalue_2 :`true` (+ _returnvalue_2 1))))
  (if (> _returnvalue_3 _returnvalue)
    (`GameplayStatics.CreatePlayer` -1)
    (goto _label)
    (elif (< _returnvalue_3 _returnvalue)
      (`GameplayStatics.RemovePlayer` (`GameplayStatics.GetPlayerController` (- _returnvalue 1)) true)
      (goto _label))))

(fn `UserConstructionScript`)