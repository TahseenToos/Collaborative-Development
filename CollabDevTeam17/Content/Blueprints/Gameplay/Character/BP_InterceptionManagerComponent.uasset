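; Player character component that starts an interception QTE against nearby players who are holding caught fish.
; InitiateInterception runs a sphere overlap, creates a QTE widget with the owner as Attacker and the target as Defender, then places it through the HUD at the target's projected screen position.
; Setup events store the widget and role, letting four directional input events forward to the matching Attacker or Defender handler.
; Tick optionally draws the detection radius for debugging.
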(event `self.ReceiveBeginPlay`
  (set `self.Show Debug Lines` false)
  (set `self.InPlay` true)
  (bind _asbp_gameplay_gamemode (cast `/Game/Blueprints/Gameplay/Gamemode/BP_GameplayGamemode` (`GameplayStatics.GetGameMode`)))
  (set `self.As BP Gameplay Gamemode` _asbp_gameplay_gamemode))

(event `self.ReceiveTick`
  (params (DeltaSeconds :type "Float (single-precision)"))
  (`self.Draw Debug Lines` DeltaSeconds))

(event `Initiate Interception`
  (bind _returnvalue (`self.GetOwner`))
  (if (not (`self.Is in Interception`))
    (bind (_outactors _returnvalue_2) (`KismetSystemLibrary.SphereOverlapActors` (`self.K2_GetComponentLocation`) (`self.Radius`) (`self.Object Types`) (`GameplayStatics.GetObjectClass` _returnvalue) (`|MakeArray` _returnvalue)))
    (if _returnvalue_2
      (for _array_element _outactors
        (bind _asbp_player_character (cast `/Game/Blueprints/Gameplay/Character/BP_PlayerCharacter` _array_element))
        (if (> (`KismetArrayLibrary.Array_Length` (`/Game/Blueprints/Gameplay/Character/BP_FishingComponent.Caught Fish Getter` (`/Game/Blueprints/Gameplay/Character/BP_PlayerCharacter.BPC_Fishing` _asbp_player_character))) 0)
          (bind _asbp_player_character_2 (cast `/Game/Blueprints/Gameplay/Character/BP_PlayerCharacter` (`self.GetOwner`)))
          (bind _returnvalue_3 (`|CreateWidget` "/Game/UI/WBP_InterceptionQTE.WBP_InterceptionQTE_C" null 0 _asbp_player_character _asbp_player_character_2))
          (`/Game/UI/WBP_TestUI.Set Interception Widget Up` (`/Game/Blueprints/Gameplay/Gamemode/BP_GameplayUIManagerComponent.HUD Tester` (`/Game/Blueprints/Gameplay/Gamemode/BP_GameplayGamemode.BP_GameplayUIManagerComponent` (`self.As BP Gameplay Gamemode`))) (`GameplayStatics.ProjectWorldToScreen` (`GameplayStatics.GetPlayerControllerFromID` 0) (`Actor.K2_GetActorLocation` _asbp_player_character)) (`GameplayStatics.ProjectWorldToScreen` (`GameplayStatics.GetPlayerControllerFromID` 0) (`Actor.K2_GetActorLocation` _asbp_player_character)) _returnvalue_3)
          (`KismetSystemLibrary.PrintString` "Hello")
          (set `self.Is in Interception` true))))))

(event `Set up Intercept Controls`
  (params (`QTE Widget` :type "/Game/UI/WBP_InterceptionQTE Object Reference") (Role :type "/Game/Blueprints/Gameplay/Enums/EInterceptionRole Enum" :default "NewEnumerator2"))
  (set `self.QTE Widget` `QTE Widget`)
  (set `self.Interception Role` Role)
  (set `self.Is in Interception` true))

(event `Undo Set up Intercept Controls`
  (params (Role :type "/Game/Blueprints/Gameplay/Enums/EInterceptionRole Enum" :default "NewEnumerator2"))
  (set `self.QTE Widget` null)
  (set `self.Interception Role` "NewEnumerator2")
  (set `self.Is in Interception` false)
  (if (`|EnumEquality` Role "NewEnumerator1")
    _))

(event `Interception Up Controls`
  (bind _qte_widget (`self.QTE Widget`))
  (if (`self.Is in Interception`)
    (switch `/Game/Blueprints/Gameplay/Enums/EInterceptionRole` (`self.Interception Role`)
      (:`NewEnumerator0`
        (`/Game/UI/WBP_InterceptionQTE.Attacker Up` _qte_widget))
      (:`NewEnumerator1`
        (`/Game/UI/WBP_InterceptionQTE.Defender Up` _qte_widget)))))

(event `Interception Down Controls`
  (bind _qte_widget (`self.QTE Widget`))
  (if (`self.Is in Interception`)
    (switch `/Game/Blueprints/Gameplay/Enums/EInterceptionRole` (`self.Interception Role`)
      (:`NewEnumerator0`
        (`/Game/UI/WBP_InterceptionQTE.Attacker  Down` _qte_widget))
      (:`NewEnumerator1`
        (`/Game/UI/WBP_InterceptionQTE.Defender Down` _qte_widget)))))

(event `Interception Left Controls`
  (bind _qte_widget (`self.QTE Widget`))
  (if (`self.Is in Interception`)
    (switch `/Game/Blueprints/Gameplay/Enums/EInterceptionRole` (`self.Interception Role`)
      (:`NewEnumerator0`
        (`/Game/UI/WBP_InterceptionQTE.Attacker  Left` _qte_widget))
      (:`NewEnumerator1`
        (`/Game/UI/WBP_InterceptionQTE.Defender Left` _qte_widget)))))

(event `Interception Right Controls`
  (bind _qte_widget (`self.QTE Widget`))
  (if (`self.Is in Interception`)
    (switch `/Game/Blueprints/Gameplay/Enums/EInterceptionRole` (`self.Interception Role`)
      (:`NewEnumerator0`
        (`/Game/UI/WBP_InterceptionQTE.Attacker  Right` _qte_widget))
      (:`NewEnumerator1`
        (`/Game/UI/WBP_InterceptionQTE.Defender Right` _qte_widget)))))

(fn `Draw Debug Lines`
  (params (Duration :type "Float (double-precision)"))
  (if (`self.Show Debug Lines`)
    (`KismetSystemLibrary.DrawDebugSphere` (`self.K2_GetComponentLocation`) (`self.Radius`) 25 (struct :`R` 1.0 :`A` 1.0) (/ Duration 5.0) 2.0 :!label _label)
    (elif (and (`self.Show Debug Lines In Game`) (`self.InPlay`))
      (goto _label))))

(fn `Owning Controller Setter`
  (params (`Owning Controller` :type "PlayerController Object Reference"))
  (set `self.Owning Controller` `Owning Controller`))