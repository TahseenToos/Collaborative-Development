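; Player boat character that routes Enhanced Input to components for boat movement and dash, fishing minigame, and interception attacks with directional quick-time events.
; Possession passes controller, character and mesh references to components, while capsule overlaps track the fishing spot used by the minigame.
; MoveActor offers camera-relative movement limited by range from the local multiplayer camera, though nothing here calls it.
; The construction script starts a looping timer for interception debug lines.
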(event `self.ReceiveBeginPlay`)

(event `self.ReceivePossessed`
  (params (NewController :type "Controller Object Reference"))
  (bind _bpc_fishing (`self.BPC_Fishing`))
  ; Sends Controller ref to fishing component
  (bind _asplayer_controller (cast `PlayerController` (`self.GetController`)))
  (`/Game/Blueprints/Gameplay/Character/BP_FishingComponent.Owning Controller Setter` _bpc_fishing _asplayer_controller)
  (`/Game/Blueprints/Gameplay/Character/BP_FishingComponent.Owning Character Setter` _bpc_fishing self)
  (set `/Game/Blueprints/Gameplay/Character/BP_BoatMovementComponent.Mesh` (`self.Mesh`) (`self.BPC_BoatMovement`)))

(event `self.CapsuleComponent.OnComponentBeginOverlap`
  (params (OverlappedComponent :type "PrimitiveComponent Object Reference") (OtherActor :type "Actor Object Reference") (OtherComp :type "PrimitiveComponent Object Reference") (OtherBodyIndex :type Integer) (bFromSweep :type Boolean) (SweepResult :type "HitResult Structure (by ref)"))
  ; Grabs fishing spot ref if close enough
  (if (== (`GameplayStatics.GetObjectClass` OtherActor) "/Game/Blueprints/Gameplay/LevelActors/BP_FishingSpot.BP_FishingSpot_C")
    (set `self.Fishing Spot` OtherActor)))

(event `EnhancedInput|/Game/Inputs/PlayerMovement/Keybinds/IA_Move`
  (params (ActionValue :type "Vector2D Structure") (ElapsedSeconds :type "Float (double-precision)") (TriggeredSeconds :type "Float (double-precision)") (InputAction :type "InputAction Object Reference" :default "/Game/Inputs/PlayerMovement/Keybinds/IA_Move.IA_Move"))
  ; Allows player movement to be controlled
  (:`Triggered`
    (`/Game/Blueprints/Gameplay/Character/BP_BoatMovementComponent.Boat Movement` (`self.BPC_BoatMovement`) ActionValue))
  (:`Started`
    (`/Game/Blueprints/Gameplay/Character/BP_BoatMovementComponent.Boat Movement Started` (`self.BPC_BoatMovement`))))

(event `self.CapsuleComponent.OnComponentEndOverlap`
  (params (OverlappedComponent :type "PrimitiveComponent Object Reference") (OtherActor :type "Actor Object Reference") (OtherComp :type "PrimitiveComponent Object Reference") (OtherBodyIndex :type Integer))
  ; Removes fishing spot if too far
  (set `self.Fishing Spot` (`self.Empty Ref`)))

(event `EnhancedInput|/Game/Inputs/Interaction/Keybinds/IA_Fish`
  (params (ActionValue :type Boolean) (ElapsedSeconds :type "Float (double-precision)") (TriggeredSeconds :type "Float (double-precision)") (InputAction :type "InputAction Object Reference" :default "/Game/Inputs/Interaction/Keybinds/IA_Fish.IA_Fish"))
  ; Activates fishing when button is pressed and near fishing spot
  (:`Started`
    (`/Game/Blueprints/Gameplay/Character/BP_FishingComponent.TriggerFishingMinigame` (`self.BPC_Fishing`) (`self.Fishing Spot`))))

(event `EnhancedInput|/Game/Inputs/Interaction/Keybinds/IA_QTETop`
  (params (ActionValue :type Boolean) (ElapsedSeconds :type "Float (double-precision)") (TriggeredSeconds :type "Float (double-precision)") (InputAction :type "InputAction Object Reference" :default "/Game/Inputs/Interaction/Keybinds/IA_QTETop.IA_QTETop"))
  (:`Started`
    (`/Game/Blueprints/Gameplay/Character/BP_InterceptionManagerComponent.Interception Up Controls` (`self.BPC_InterceptionManager`))))

(event `EnhancedInput|/Game/Inputs/Interaction/Keybinds/IA_QTEBottom`
  (params (ActionValue :type Boolean) (ElapsedSeconds :type "Float (double-precision)") (TriggeredSeconds :type "Float (double-precision)") (InputAction :type "InputAction Object Reference" :default "/Game/Inputs/Interaction/Keybinds/IA_QTEBottom.IA_QTEBottom"))
  (:`Started`
    (`/Game/Blueprints/Gameplay/Character/BP_InterceptionManagerComponent.Interception Down Controls` (`self.BPC_InterceptionManager`))))

(event `EnhancedInput|/Game/Inputs/PlayerMovement/Keybinds/IA_Dash`
  (params (ActionValue :type Boolean) (ElapsedSeconds :type "Float (double-precision)") (TriggeredSeconds :type "Float (double-precision)") (InputAction :type "InputAction Object Reference" :default "/Game/Inputs/PlayerMovement/Keybinds/IA_Dash.IA_Dash"))
  ; Dash
  (:`Triggered`
    (`/Game/Blueprints/Gameplay/Character/BP_BoatMovementComponent.Dash` (`self.BPC_BoatMovement`))))

(event `EnhancedInput|/Game/Inputs/Interaction/Keybinds/IA_QTELeft`
  (params (ActionValue :type Boolean) (ElapsedSeconds :type "Float (double-precision)") (TriggeredSeconds :type "Float (double-precision)") (InputAction :type "InputAction Object Reference" :default "/Game/Inputs/Interaction/Keybinds/IA_QTELeft.IA_QTELeft"))
  (:`Started`
    (`/Game/Blueprints/Gameplay/Character/BP_InterceptionManagerComponent.Interception Left Controls` (`self.BPC_InterceptionManager`))))

(event `EnhancedInput|/Game/Inputs/Interaction/Keybinds/IA_FishQTE`
  (params (ActionValue :type Boolean) (ElapsedSeconds :type "Float (double-precision)") (TriggeredSeconds :type "Float (double-precision)") (InputAction :type "InputAction Object Reference" :default "/Game/Inputs/Interaction/Keybinds/IA_FishQTE.IA_FishQTE"))
  ; Fishing Quick-time-event
  (:`Started`
    (`/Game/Blueprints/Gameplay/Character/BP_FishingComponent.FishingQTE pressed` (`self.BPC_Fishing`))))

(event `EnhancedInput|/Game/Inputs/Interaction/Keybinds/IA_QTERight`
  (params (ActionValue :type Boolean) (ElapsedSeconds :type "Float (double-precision)") (TriggeredSeconds :type "Float (double-precision)") (InputAction :type "InputAction Object Reference" :default "/Game/Inputs/Interaction/Keybinds/IA_QTERight.IA_QTERight"))
  (:`Started`
    (`/Game/Blueprints/Gameplay/Character/BP_InterceptionManagerComponent.Interception Right Controls` (`self.BPC_InterceptionManager`))))

(event `EnhancedInput|/Game/Inputs/Interaction/Keybinds/IA_Attack`
  (params (ActionValue :type Boolean) (ElapsedSeconds :type "Float (double-precision)") (TriggeredSeconds :type "Float (double-precision)") (InputAction :type "InputAction Object Reference" :default "/Game/Inputs/Interaction/Keybinds/IA_Attack.IA_Attack"))
  ; Triggers interception mechanic if player is within range
  (:`Started`
    (`/Game/Blueprints/Gameplay/Character/BP_InterceptionManagerComponent.Initiate Interception` (`self.BPC_InterceptionManager`))))

(fn `Draw Debug Lines For Interception`
  (`/Game/Blueprints/Gameplay/Character/BP_InterceptionManagerComponent.Draw Debug Lines` (`self.BPC_InterceptionManager`) 0.01))

(fn `Move Actor`
  (params (`X Axis` :type "Float (double-precision)") (`Y Axis` :type "Float (double-precision)"))
  (bind _local_multiplayer_camera (`self.Local Multiplayer Camera`))
  (bind _local_multiplayer_camera_2 (`self.Local Multiplayer Camera`))
  (bind (_returnvalue_roll _returnvalue_pitch _returnvalue_yaw) (`KismetMathLibrary.BreakRotator` (`SceneComponent.K2_GetComponentRotation` (`/Game/Blueprints/Camera/BP_LocalMultiplayerCamera.Camera` (`self.Local Multiplayer Camera`)))))
  (bind (_returnvalue_roll_2 _returnvalue_pitch_2 _returnvalue_yaw_2) (`KismetMathLibrary.BreakRotator` (`SceneComponent.K2_GetComponentRotation` (`/Game/Blueprints/Camera/BP_LocalMultiplayerCamera.Camera` (`self.Local Multiplayer Camera`)))))
  (bind _returnvalue (`KismetMathLibrary.Dot_VectorVector` (- (`self.K2_GetActorLocation` _local_multiplayer_camera_2) (`self.K2_GetActorLocation`)) (`KismetMathLibrary.GetUpVector` (`SceneComponent.K2_GetComponentRotation` (`/Game/Blueprints/Camera/BP_LocalMultiplayerCamera.Camera` _local_multiplayer_camera_2)))))
  (bind _returnvalue_2 (`KismetMathLibrary.Dot_VectorVector` (- (`self.K2_GetActorLocation` _local_multiplayer_camera) (`self.K2_GetActorLocation`)) (`KismetMathLibrary.GetRightVector` (`SceneComponent.K2_GetComponentRotation` (`/Game/Blueprints/Camera/BP_LocalMultiplayerCamera.Camera` _local_multiplayer_camera)))))
  (`|ExecutionSequence`
    (:`then_0`
      (`self.Local Multiplayer Camera`
        (:`then`)
        (:`else`
          (bind _returnvalue_3 (`GameplayStatics.GetActorOfClass` "/Game/Blueprints/Camera/BP_LocalMultiplayerCamera.BP_LocalMultiplayerCamera_C"))
          (set `self.Local Multiplayer Camera` _returnvalue_3))))
    (:`then_1`
      (`self.AddMovementInput` (`KismetMathLibrary.GetRightVector` (`KismetMathLibrary.MakeRotator` _returnvalue_roll 0.0 _returnvalue_yaw)) (`KismetMathLibrary.SelectFloat` (`local.X Axis`) 0.0 (or (< (`KismetMathLibrary.Abs` _returnvalue_2) (`self.Max X Movement Range From Camera`)) (and (> _returnvalue_2 0.0) (> (`local.X Axis`) 0.0)) (and (< _returnvalue_2 0.0) (< (`local.X Axis`) 0.0)))))
      (`self.AddMovementInput` (`KismetMathLibrary.GetForwardVector` (`KismetMathLibrary.MakeRotator` 0.0 0.0 _returnvalue_yaw_2)) (`KismetMathLibrary.SelectFloat` (`local.Y Axis`) 0.0 (or (< (`KismetMathLibrary.Abs` _returnvalue) (`self.Max Y Movement Range From Camera`)) (and (> _returnvalue 0.0) (> (`local.Y Axis`) 0.0)) (and (< _returnvalue 0.0) (< (`local.Y Axis`) 0.0))))))))

(fn `UserConstructionScript`
  (locals (`Debug Lines Timer Handler` :type "TimerHandle Structure") (`Time between drawing lines` :type "Float (single-precision)" :default 0.01))
  (`KismetSystemLibrary.K2_ClearAndInvalidateTimerHandle` (`local.Debug Lines Timer Handler`))
  (bind _returnvalue (`KismetSystemLibrary.K2_SetTimer` null "Draw Debug Lines For Interception" (`local.Time between drawing lines`) true))
  (set `local.Debug Lines Timer Handler` _returnvalue))