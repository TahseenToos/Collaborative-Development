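; Scene component on player characters that manages interception quick-time events between an attacker and nearby defenders.
; On initiation, it sphere-overlaps for other actors of the owner's class and creates a QTE widget per player found, with the owner as attacker.
; Once given a widget and role, it forwards directional inputs to that widget's attacker or defender functions.
; Optional debug drawing shows the detection radius each tick.
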(event `self.ReceiveBeginPlay`
  (set `self.Show Debug Lines` false)
  (set `self.InPlay` true))

(event `self.ReceiveTick`
  (params (DeltaSeconds :type "Float (single-precision)"))
  (`self.Draw Debug Lines` DeltaSeconds))

(event `Initiate Interception`
  (bind _returnvalue (`self.GetOwner`))
  (bind (_outactors _returnvalue_2) (`KismetSystemLibrary.SphereOverlapActors` (`self.K2_GetComponentLocation`) (`self.Radius`) (`self.Object Types`) (`GameplayStatics.GetObjectClass` _returnvalue) (`|MakeArray` _returnvalue)))
  (if _returnvalue_2
    (for _array_element _outactors
      (bind _asbp_player_character (cast `/Game/Blueprints/Gameplay/Character/BP_PlayerCharacter` _array_element)
        (:`then`
          (bind _asbp_player_character_2 (cast `/Game/Blueprints/Gameplay/Character/BP_PlayerCharacter` (`self.GetOwner`)))
          (`|CreateWidget` "/Game/Blueprints/InterceptionQTE/WBP_InterceptionQTE.WBP_InterceptionQTE_C" null 0 _asbp_player_character _asbp_player_character_2))
        (:`CastFailed`
          (`KismetSystemLibrary.PrintString` "ooopsie"))))
    (else
      (`KismetSystemLibrary.PrintString` "boohoo"))))

(event `/Game/Blueprints/Gameplay/Interface/I_Request_QTE_Setup.Set up Intercept Controls`
  (params (`QTE Widget` :type "/Game/Blueprints/InterceptionQTE/WBP_InterceptionQTE Object Reference") (Role :type "/Game/Blueprints/Gameplay/Enums/E_InterceptionRole Enum" :default "NewEnumerator0"))
  (set `self.QTE Widget` `QTE Widget`)
  (set `self.Interception Role` Role))

(event `Interception Up Controls`
  (bind _qte_widget (`self.QTE Widget`))
  (switch `/Game/Blueprints/Gameplay/Enums/E_InterceptionRole` (`self.Interception Role`)
    (:`NewEnumerator0`
      (`/Game/Blueprints/InterceptionQTE/WBP_InterceptionQTE.Attacker Up` _qte_widget))
    (:`NewEnumerator1`
      (`/Game/Blueprints/InterceptionQTE/WBP_InterceptionQTE.Defender Up` _qte_widget))))

(event `Interception Down Controls`
  (bind _qte_widget (`self.QTE Widget`))
  (switch `/Game/Blueprints/Gameplay/Enums/E_InterceptionRole` (`self.Interception Role`)
    (:`NewEnumerator0`
      (`/Game/Blueprints/InterceptionQTE/WBP_InterceptionQTE.Attacker  Down` _qte_widget))
    (:`NewEnumerator1`
      (`/Game/Blueprints/InterceptionQTE/WBP_InterceptionQTE.Defender Down` _qte_widget))))

(event `Interception Left Controls`
  (bind _qte_widget (`self.QTE Widget`))
  (switch `/Game/Blueprints/Gameplay/Enums/E_InterceptionRole` (`self.Interception Role`)
    (:`NewEnumerator0`
      (`/Game/Blueprints/InterceptionQTE/WBP_InterceptionQTE.Attacker  Left` _qte_widget))
    (:`NewEnumerator1`
      (`/Game/Blueprints/InterceptionQTE/WBP_InterceptionQTE.Defender Left` _qte_widget))))

(event `Interception Right Controls`
  (bind _qte_widget (`self.QTE Widget`))
  (switch `/Game/Blueprints/Gameplay/Enums/E_InterceptionRole` (`self.Interception Role`)
    (:`NewEnumerator0`
      (`/Game/Blueprints/InterceptionQTE/WBP_InterceptionQTE.Attacker  Right` _qte_widget))
    (:`NewEnumerator1`
      (`/Game/Blueprints/InterceptionQTE/WBP_InterceptionQTE.Defender Right` _qte_widget))))

(fn `Draw Debug Lines`
  (params (Duration :type "Float (double-precision)"))
  (if (`self.Show Debug Lines`)
    (`KismetSystemLibrary.DrawDebugSphere` (`self.K2_GetComponentLocation`) (`self.Radius`) 25 (struct :`R` 1.0 :`A` 1.0) (/ Duration 5.0) 2.0 :!label _label)
    (elif (and (`self.Show Debug Lines In Game`) (`self.InPlay`))
      (goto _label))))

(fn `Owning Controller Setter`
  (params (`Owning Controller` :type "PlayerController Object Reference"))
  (set `self.Owning Controller` `Owning Controller`))