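; Character fishing component that runs the fishing QTE minigame and holds the player's caught fish.
; It messages a fishing spot when not already fishing, then shows a QTE widget built from the fish info on the character's widget component.
; Presses are forwarded to that widget, and success stores the fish and clears it.
; DepositFish returns from inside its loop, reporting only the first fish's points with the owning controller.
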(event Custom|Start%20Fishing%20QTE
  (params (Fish%20Info :type S%20Fish%20Stats%20Structure))
  (bind _owning_controller (Variables|Default|GetOwning%20Controller))
  (Variables|Default|SetCaught%20Fish%20Info (.CaughtFishInfo (Utilities|Struct|BreakSFishStats Fish%20Info)))
  (Utilities|IsValid _owning_controller
    (:Is%20Valid
      (bind _returnvalue (UserInterface|CreateWidget "/Game/UI/UI_FishingDisplay.UI_FishingDisplay_C" _owning_controller Fish%20Info))
      (bind _output_get (Variables|Default|SetFishingQTEUI _returnvalue))
      (UserInterface|SetWidget (Variables|/Game/Blueprints/Gameplay/Character/BP_PlayerCharacter.BP_PlayerCharacter_C|GetWBP_FishingQTEComponent (Variables|Default|GetCharacter)) _output_get)
      (Variables|Default|SetIsAlreadyFishing true))))

(event Custom|TriggerFishingMinigame
  (params (FishingSpot :type Actor%20Object%20Reference))
  ;[0.15 0.15 0.15 0.5] Calls interface event for fishing spot
  (if (not (Variables|Default|GetIsAlreadyFishing))
    (Class|BPIFishing|Fishing(Message) FishingSpot self)))

(event Custom|Fishing%20Successful
  (params (Fish%20Caught :type S%20Caught%20Fish%20Structure))
  (CallFunction|AddFishtoInventory Fish%20Caught)
  (Development|PrintString "added fish")
  (Variables|Default|SetIsAlreadyFishing false)
  (UserInterface|SetWidget (Variables|/Game/Blueprints/Gameplay/Character/BP_PlayerCharacter.BP_PlayerCharacter_C|GetWBP_FishingQTEComponent (Variables|Default|GetCharacter)) 0))

(event Custom|FishingQTE%20pressed
  (Class|BPIFishing|FishingQTE(Message) (Variables|Default|GetFishingQTEUI) self))

(event EventBeginPlay)

(event EventTick
  (params (DeltaSeconds :type Float%20%28single-precision%29)))

(event Input|KeyboardEvents|DebugKeyM
  (params (Key :type Key%20Structure :default "None") (ActionValue :type Input%20Action%20Value%20Structure))
  (:Pressed
    (for _array_element (Variables|Default|GetCaught%20Fish)
      (Development|PrintString (Utilities|String|ToString(Name) (.FishName (Utilities|Struct|BreakSCaughtFish _array_element)))))))

(fn OwningControllerSetter
  (params (Controller :type Player%20Controller%20Object%20Reference))
  (Variables|Default|SetOwning%20Controller Controller))

(fn CaughtFishGetter
  (return (Variables|Default|GetCaught%20Fish)))

(fn AddFishtoInventory
  (params (Fish :type S%20Caught%20Fish%20Structure))
  (Utilities|Array|Add (Variables|Default|GetCaught%20Fish) Fish))

(fn RemoveFishfromInventory
  (params (Fish%20Index :type Integer))
  (Utilities|Array|RemoveIndex (Variables|Default|GetCaught%20Fish) Fish%20Index))

(fn DepositFish
  (for _array_element (Variables|Default|GetCaught%20Fish)
    (bind _output_get (LocalVariables|SetTotal%20Fish%20Score (.Points (Utilities|Struct|BreakSCaughtFish _array_element))))
    (return _output_get (Variables|Default|GetOwning%20Controller))))

(fn OwningCharacterSetter
  (params (Character :type BP%20Player%20Character%20Object%20Reference))
  (Variables|Default|SetCharacter Character))