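; Character component that runs the fishing minigame and keeps the list of fish the player has caught.
; It messages a fishing spot to begin, then shows a fishing QTE widget built from the given fish info on the owning controller.
; QTE presses are forwarded to that widget through an interface, and successful catches are stored.
; A busy flag blocks retriggering until a catch succeeds, and a debug key prints caught fish names.
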(event Custom|Start%20Fishing%20QTE
  (params (Fish%20Info :type S%20Fish%20Stats%20Structure))
  (bind _owning_controller (Variables|Default|GetOwning%20Controller))
  (Variables|Default|SetCaught%20Fish%20Info (.CaughtFishInfo (Utilities|Struct|BreakS_FishStats Fish%20Info)))
  (Utilities|IsValid _owning_controller
    (:Is%20Valid
      (bind _returnvalue (UserInterface|CreateWidget "/Game/UI/UI_FishingDisplay.UI_FishingDisplay_C" _owning_controller Fish%20Info))
      (bind _output_get (Variables|Default|SetFishingQTEUI _returnvalue))
      (UserInterface|Viewport|AddtoViewport _output_get 0)
      (Variables|Default|SetIsAlreadyFishing true))))

(event Custom|TriggerFishingMinigame
  (params (FishingSpot :type Actor%20Object%20Reference))
  ;[0.15 0.15 0.15 0.5] Calls interface event for fishing spot
  (if (not (Variables|Default|GetIsAlreadyFishing))
    (Class|IFishing|Fishing(Message) FishingSpot self)))

(event Custom|Fishing%20Successful
  (params (Fish%20Caught :type S%20Caught%20Fish%20Structure))
  (Utilities|Array|Add (Variables|Default|GetCaught%20Fish) Fish%20Caught)
  (Development|PrintString "added fish")
  (Variables|Default|SetIsAlreadyFishing false))

(event Custom|FishingQTE%20pressed
  (Class|IFishing|FishingQTE(Message) (Variables|Default|GetFishingQTEUI) self))

(event EventBeginPlay)

(event EventTick
  (params (DeltaSeconds :type Float%20%28single-precision%29)))

(event Input|KeyboardEvents|DebugKeyM
  (params (Key :type Key%20Structure :default "None") (ActionValue :type Input%20Action%20Value%20Structure))
  (:Pressed
    (for _array_element (Variables|Default|GetCaught%20Fish)
      (Development|PrintString (Utilities|String|ToString(Name) (.FishName (Utilities|Struct|BreakS_CaughtFish _array_element)))))))

(fn OwningControllerSetter
  (params (Controller :type Player%20Controller%20Object%20Reference))
  (Variables|Default|SetOwning%20Controller Controller))

(fn CaughtFishGetter
  (return (Variables|Default|GetCaught%20Fish)))