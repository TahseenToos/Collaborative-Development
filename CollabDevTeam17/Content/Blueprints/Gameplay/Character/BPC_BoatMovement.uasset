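; Boat movement component that handles steering, leaning and dashing for the player's boat.
; Enhanced Input turns the pawn gradually toward the stick direction and adds movement input along it.
; The mesh leans by the dot product of input and right vector, and Tick eases it toward a target that zeroes on release.
; A DoOnce-gated dash launches the Character forward, then kicks it upward shortly after, before a cooldown.
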(event `EnhancedInput|/Game/Inputs/PlayerMovement/Keybinds/IA_Movement`
  (params (ActionValue :type "Vector2D Structure") (ElapsedSeconds :type "Float (double-precision)") (TriggeredSeconds :type "Float (double-precision)") (InputAction :type "InputAction Object Reference" :default "/Game/Inputs/PlayerMovement/Keybinds/IA_Movement.IA_Movement"))
  (bind (_x _y) (`KismetMathLibrary.BreakVector2D` ActionValue))
  (bind _returnvalue (`KismetMathLibrary.Normal` (`KismetMathLibrary.MakeVector` _y _x)))
  (bind _returnvalue_2 (`KismetMathLibrary.Dot_VectorVector` _returnvalue (`Actor.GetActorRightVector` (`Actor.Instigator` (`self.GetOwner`)))))
  (bind _returnvalue_3 (* _returnvalue_2 (`self.MaxLeanAngle`)))
  ; Movement
  (:`Triggered`
    (`Actor.K2_SetActorRotation` (`Actor.Instigator` (`self.GetOwner`)) (`KismetMathLibrary.RInterpTo` (`Actor.K2_GetActorRotation` (`Actor.Instigator` (`self.GetOwner`))) (`KismetMathLibrary.MakeRotFromX` _returnvalue) (`GameplayStatics.GetWorldDeltaSeconds`) 3.0) false)
    (set `self.TargetLean` _returnvalue_2)
    (set `self.CurrentLean` _returnvalue_3)
    (`SceneComponent.K2_SetRelativeRotation` (`self.Mesh`) (`KismetMathLibrary.MakeRotator` 0.0 _returnvalue_3 -90.0) false false)
    (`Pawn.AddMovementInput` (`Actor.Instigator` (`self.GetOwner`)) _returnvalue 1.0 false))
  (:`Canceled`
    (set `self.TargetLean` 0.0)))

(event `self.ReceiveTick`
  (params (DeltaSeconds :type "Float (single-precision)"))
  (bind _returnvalue (`KismetMathLibrary.FInterpTo` (`self.CurrentLean`) (`self.TargetLean`) (`GameplayStatics.GetWorldDeltaSeconds`) 3.0))
  ; Tilt Back To Normal When Idle
  (set `self.CurrentLean` _returnvalue)
  (`SceneComponent.K2_SetRelativeRotation` (`self.Mesh`) (`KismetMathLibrary.MakeRotator` 0.0 _returnvalue -90.0) false false))

(event `EnhancedInput|/Game/Inputs/PlayerMovement/Keybinds/IA_Dash`
  (params (ActionValue :type Boolean) (ElapsedSeconds :type "Float (double-precision)") (TriggeredSeconds :type "Float (double-precision)") (InputAction :type "InputAction Object Reference" :default "/Game/Inputs/PlayerMovement/Keybinds/IA_Dash.IA_Dash"))
  (bind _returnvalue (`Actor.K2_GetActorRotation` (`Actor.Instigator` (`self.GetOwner`))))
  ; Dash
  (:`Triggered`
    (`/Engine/EditorBlueprintResources/StandardMacros.DoOnce` false :!label _label
      (:`Completed`
        (bind _ascharacter (cast `Character` (`self.GetOwner`)))
        (`Character.LaunchCharacter` _ascharacter (* (`KismetMathLibrary.GetForwardVector` _returnvalue) (`self.DashMultiplier`)) false false)
        (`KismetSystemLibrary.Delay` 0.1)
        (`Character.LaunchCharacter` _ascharacter (* (`KismetMathLibrary.GetUpVector` _returnvalue) (`self.DashKickUp`)) false false)
        (`KismetSystemLibrary.Delay` (`self.DashCooldown`))
        (goto _label :!via `Reset`)))))