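; Sea mine level actor that stuns a boat on contact and knocks it away from the mine.
; At BeginPlay it registers with the gamemode's sea mine manager component, then starts hidden with collision disabled.
; On overlap it calls Stun on the boat movement component and applies a horizontal impulse scaled by Knockback.
; It then disables itself and reports back to the manager as an available mine.
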(event `self.ReceiveBeginPlay`
  ; Sets up mines initally.
  (bind _asbp_gameplay_gamemode (cast `/Game/Blueprints/Gameplay/Gamemode/BP_GameplayGamemode` (`GameplayStatics.GetGameMode`)))
  (bind _output_get (set `self.GamemodeReference` _asbp_gameplay_gamemode))
  (`/Game/Blueprints/Gameplay/Gamemode/BPC_SeaMineManagerComponent.OnRegisterMineLocation` (`/Game/Blueprints/Gameplay/Gamemode/BP_GameplayGamemode.BPC_SeaMineManagerComponent` _output_get) self)
  (`self.SetActorHiddenInGame` self true)
  (`self.SetActorEnableCollision` self false))

(event `OnDisableMine`
  ; Hides the mine after it is collided with.
  (`self.SetActorHiddenInGame` true)
  (`self.SetActorEnableCollision` false)
  (`/Game/Blueprints/Gameplay/Gamemode/BPC_SeaMineManagerComponent.IncreaseAvailableMines` (`/Game/Blueprints/Gameplay/Gamemode/BP_GameplayGamemode.BPC_SeaMineManagerComponent` (`self.GamemodeReference`)) self))

(event `self.ReceiveActorBeginOverlap`
  (params (OtherActor :type "Actor Object Reference"))
  (bind _returnvalue (`SceneComponent.K2_GetComponentToWorld` (`self.DefaultSceneRoot`)))
  (bind _returnvalue_2 (`SceneComponent.K2_GetComponentToWorld` (`Actor.RootComponent` (`self.CollidedWithPlayer`))))
  (bind _returnvalue_3 (* (`KismetMathLibrary.Normal` (- (`KismetMathLibrary.MakeVector` (.x (.location _returnvalue_2)) (.y (.location _returnvalue_2))) (`KismetMathLibrary.MakeVector` (.x (.location _returnvalue)) (.y (.location _returnvalue)))) 1.0) (`self.Knockback`)))
  ; Colliding with sea mine behaviour.
  ;; Sets up variables/calls
  (set `self.CollidedWithPlayer` OtherActor)
  ;; Stuns the player and impulses a velocity away from the seamine location.
  (`/Game/Blueprints/Gameplay/Character/BP_BoatMovementComponent.Stun` (`self.GetComponentByClass` OtherActor "/Game/Blueprints/Gameplay/Character/BP_BoatMovementComponent.BP_BoatMovementComponent_C"))
  (`KismetSystemLibrary.PrintString` (`KismetStringLibrary.BuildString_Vector` "Knockback impulse is " "" _returnvalue_3))
  (`CharacterMovementComponent.AddImpulse` (`self.GetComponentByClass` OtherActor "/Script/Engine.CharacterMovementComponent") _returnvalue_3 true)
  (`self.OnDisableMine`))

(fn `UserConstructionScript`)