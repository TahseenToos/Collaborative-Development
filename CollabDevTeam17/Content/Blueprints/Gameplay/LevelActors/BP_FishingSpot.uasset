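; BP_FishingSpot is a level actor that players can fish at while it is active, one at a time.
; A capsule tracks nearby players, and fishing starts that player's QTE with a fish picked randomly from a catalogue on activation.
; Activation and deactivation toggle mesh material and water VFX, with deactivation also ending nearby players' QTEs.
; A timeline flickers the material as a warning before deactivation, while a successful catch asks the manager to swap spots.
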(event `self.ReceiveBeginPlay`
  ; Sets default material on BeginPlay
  (bind _output_get (set `self.Default Mat` (`PrimitiveComponent.GetMaterial` (`self.FishingSpotMesh`) 0)))
  (`KismetMaterialLibrary.CreateDynamicMaterialInstance` _output_get)
  (`|CreateWidget` "/Game/UI/CurrentUIWork/WBP_PopupForInRadius.WBP_PopupForInRadius_C"))

(event `Successfully Fished`
  (`/Game/Blueprints/Gameplay/Gamemode/BP_FishingSpotManagerComponent.Swap Fishing Spots` (`self.Manager`) self))

(event `self.Capsule.OnComponentBeginOverlap`
  (params (OverlappedComponent :type "PrimitiveComponent Object Reference") (OtherActor :type "Actor Object Reference") (OtherComp :type "PrimitiveComponent Object Reference") (OtherBodyIndex :type Integer) (bFromSweep :type Boolean) (SweepResult :type "HitResult Structure (by ref)"))
  ; Sorts reference to all players close to it
  (if (`self.Is Active`)
    (bind _asbp_player_character (cast `/Game/Blueprints/Gameplay/Character/BP_PlayerCharacter` OtherActor))
    (`KismetArrayLibrary.Array_AddUnique` (`self.PlayersNearFishingSpot`) _asbp_player_character)))

(event `self.Capsule.OnComponentEndOverlap`
  (params (OverlappedComponent :type "PrimitiveComponent Object Reference") (OtherActor :type "Actor Object Reference") (OtherComp :type "PrimitiveComponent Object Reference") (OtherBodyIndex :type Integer))
  ; Sorts reference to all players close to it
  (if (`self.Is Active`)
    (bind _asbp_player_character (cast `/Game/Blueprints/Gameplay/Character/BP_PlayerCharacter` OtherActor))
    (`KismetArrayLibrary.Array_RemoveItem` (`self.PlayersNearFishingSpot`) _asbp_player_character)))

(event `/Game/Blueprints/Gameplay/Interface/BPI_Fishing.Fishing`
  (params (PlayerFishing :type "/Game/Blueprints/Gameplay/Character/BP_FishingComponent Object Reference"))
  ; Activates fishing in the player
  (if (and (`self.Is Active`) (`self.Not Being Fished`))
    (set `self.Not Being Fished` false)
    (`/Game/Blueprints/Gameplay/Character/BP_FishingComponent.Start Fishing QTE` PlayerFishing (`self.FishToBeCaught`))))

(event `Deactivation Warning`
  (`Timeline|Fishing Spot Deactivating` :!via `PlayFromStart`
    (:`Finished`
      (`self.Deactivate Fishing Spot`))
    (:`Change Material`
      (`/Engine/EditorBlueprintResources/StandardMacros.FlipFlop`
        (:`A`
          (`PrimitiveComponent.SetMaterial` (`self.FishingSpotMesh`) 0 (`self.Default Mat`)))
        (:`B`
          (`PrimitiveComponent.SetMaterial` (`self.FishingSpotMesh`) 0 "/Engine/Engine_MI_Shaders/Instances/M_Shader_SimpleTranslucent_Invis.M_Shader_SimpleTranslucent_Invis"))))))

(event `Activate Fishing Spot`
  ; Activates spot to be fishable
  (set `self.Is Active` true)
  (`PrimitiveComponent.SetMaterial` (`self.FishingSpotMesh`) 0 "/Engine/Engine_MI_Shaders/Instances/M_Shader_SimpleTranslucent_Invis.M_Shader_SimpleTranslucent_Invis")
  (`ActorComponent.Activate` (`self.WaterVFX`) false)
  (set `self.FishToBeCaught` (`KismetArrayLibrary.Array_Random` (`self.Fish Catalogue`))))

(event `Deactivate Fishing Spot`
  ; Deactivates spot to no longer be fishable
  (set `self.Is Active` false)
  (`PrimitiveComponent.SetMaterial` (`self.FishingSpotMesh`) 0 (`self.Default Mat`))
  (`ActorComponent.Deactivate` (`self.WaterVFX`))
  (for _array_element (`self.PlayersNearFishingSpot`)
    (`/Game/Blueprints/Gameplay/Character/BP_FishingComponent.End Fishing QTE` (`/Game/Blueprints/Gameplay/Character/BP_PlayerCharacter.BPC_Fishing` _array_element) false))
  (`KismetArrayLibrary.Array_Clear` (`self.PlayersNearFishingSpot`)))

(event `End Fishing`
  (set `self.Not Being Fished` true))

(fn `UserConstructionScript`)