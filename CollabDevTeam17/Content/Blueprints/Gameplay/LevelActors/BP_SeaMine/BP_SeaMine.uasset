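; BP_SeaMine is a level hazard that stuns and knocks back a boat that overlaps it.
; On overlap it calls Stun on the BP_BoatMovementComponent, then impulses the CharacterMovementComponent as a velocity change.
; The impulse is the horizontal mine-to-player offset, unnormalized, inverse-transformed into player space and scaled by Knockback.
; Each mine adds itself to MineArray on BeginPlay, but random activation and disabling after a hit are unimplemented stubs.
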(event `self.ReceiveBeginPlay`
  ; Sets up mines initally.
  (`self.OnRegisterMineLocation`)
  (`self.OnEnableMine`))

(event `OnEnableMine`
  ; Meant to get random mines activated.
  (if (> (`self.MineCount`) 0)
    _))

(event `OnRegisterMineLocation`
  ; Registers mines to an array to store their locations.
  (`KismetArrayLibrary.Array_Add` (`self.MineArray`) self))

(event `self.ReceiveActorBeginOverlap`
  (params (OtherActor :type "Actor Object Reference"))
  (bind _returnvalue (`SceneComponent.K2_GetComponentToWorld` (`Actor.RootComponent` (`self.CollidedWithPlayer`))))
  (bind _returnvalue_2 (`SceneComponent.K2_GetComponentToWorld` (`self.DefaultSceneRoot`)))
  ; Colliding with sea mine behaviour.
  ;; Sets up variables/calls
  (set `self.CollidedWithPlayer` OtherActor)
  ;; Stuns the player and impulses a velocity away from the seamine location.
  (`/Game/Blueprints/Gameplay/Character/BP_BoatMovementComponent.Stun` (`self.GetComponentByClass` OtherActor "/Game/Blueprints/Gameplay/Character/BP_BoatMovementComponent.BP_BoatMovementComponent_C"))
  (`CharacterMovementComponent.AddImpulse` (`self.GetComponentByClass` OtherActor "/Script/Engine.CharacterMovementComponent") (* (`self.Knockback`) (`KismetMathLibrary.InverseTransformDirection` (`SceneComponent.K2_GetComponentToWorld` (`Actor.RootComponent` (`self.CollidedWithPlayer`))) (- (`KismetMathLibrary.MakeVector` (.x (.location _returnvalue)) (.y (.location _returnvalue))) (`KismetMathLibrary.MakeVector` (.x (.location _returnvalue_2)) (.y (.location _returnvalue_2)))))) true)
  (`self.OnDisableMine`))

(event `OnDisableMine`)

(fn `UserConstructionScript`)