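; BP_PlayerSpawnpoint is a level actor that positions a player character at its transform once players have spawned.
; On BeginPlay it caches BP_GameplayGamemode and binds to its OnPlayersSpawned event.
; SpawnPlayerHere creates no pawn: it teleports the first BP_PlayerCharacter not yet flagged AtSpawnpoint, then sets that flag, so each spawnpoint claims a different player.
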(event `self.ReceiveBeginPlay`
  (bind _asbp_gameplay_gamemode (cast `/Game/Blueprints/Gameplay/Gamemode/BP_GameplayGamemode` (`GameplayStatics.GetGameMode`)))
  (bind _output_get (set `self.Gamemode` _asbp_gameplay_gamemode))
  (add `/Game/Blueprints/Gameplay/Gamemode/BP_GameplayGamemode.On Players Spawned` _output_get (`|CreateDelegate` :!event `Spawn Player Here`)))

(event `Spawn Player Here`
  (bind _outactors (`GameplayStatics.GetAllActorsOfClass` "/Game/Blueprints/Gameplay/Character/BP_PlayerCharacter.BP_PlayerCharacter_C"))
  (for _array_element _outactors
    (if (not (`/Game/Blueprints/Gameplay/Character/BP_PlayerCharacter.At Spawnpoint` _array_element))
      (`self.K2_SetActorTransform` _array_element (`self.GetTransform`) false true)
      (set `/Game/Blueprints/Gameplay/Character/BP_PlayerCharacter.At Spawnpoint` true _array_element)
      (break))))

(fn `UserConstructionScript`)