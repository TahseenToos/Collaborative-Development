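; BP_Goal_Manager is a prototype manager that handles goal collisions and scoring.
; GoalCollision prints the player and goal, then calls IncreasePlayerScore, which adds one to a single CurrentPlayerScore, reset to zero on BeginPlay, and prints the total.
; Per-player scoring and fish values are noted as intended but absent.
; EndGameplayCountdown is an empty stub, and the placeholder winner message is never run.
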(event `self.ReceiveBeginPlay`
  ; Intended to set all player scores to zero.
  (set `self.Current Player Score` 0.0))

(event `/Game/Blueprints/Gameplay/TimerAndGoal/I_Goal_Interface.Goal Collision`
  (params (Player :type "/Game/Blueprints/Gameplay/Character/BP_PlayerCharacter Object Reference") (Goal :type "/Game/Blueprints/Gameplay/TimerAndGoal/BP_Goal Object Reference"))
  ; Goal collision handler. Triggers the "Increases player score" section.
  ;; When a goal is collided with.
  ;; Intended to get: the goal, the player and the fish the player has.
  (`KismetSystemLibrary.PrintString` (`KismetStringLibrary.Concat_StrStr` (`KismetSystemLibrary.GetDisplayName` Player) " collided with " (`KismetSystemLibrary.GetDisplayName` Goal)))
  ;; Trigger the increase of the player score here.
  (`self.Increase Player Score` Player))

(event `Increase Player Score`
  (params (Player :type "/Game/Blueprints/Gameplay/Character/BP_PlayerCharacter Object Reference"))
  ; Increases player score.
  ;; When the player score event is triggered
  ;; Intended to add fish score value to player score. Need to replace.
  (bind _output_get (set `self.Current Player Score` (+ (`self.Current Player Score`) 1.0)))
  ;; Announces player score (for debug reasons, also replace later with UI).
  (`KismetSystemLibrary.PrintString` (`KismetStringLibrary.BuildString_Double` "" (`KismetStringLibrary.Concat_StrStr` (`KismetSystemLibrary.GetDisplayName` Player) "[Player Number goes here]" (`self.Score String`)) _output_get)))

(event `End Gameplay Countdown`
  ; This section is to find the winner. Multiplayer required to do this.
)