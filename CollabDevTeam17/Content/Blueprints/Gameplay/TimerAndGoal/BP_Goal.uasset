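; BP_Goal is a fish drop-off goal that scores fish the player deposits by entering its box collider.
; On overlap, the player's fishing component deposits fish of the accepted type, and the resulting score and character go to the gamemode's goal manager component.
; With random goals enabled, it registers with the timer manager at BeginPlay.
; The event for changing the accepted type is empty, with its randomization logic left disconnected.
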(event `self.ReceiveBeginPlay`
  ; Sets up the goal at the start.
  (bind _asbp_gameplay_gamemode (cast `/Game/Blueprints/Gameplay/Gamemode/BP_GameplayGamemode` (`GameplayStatics.GetGameMode`)))
  (bind _output_get (set `self.As BP Gameplay Gamemode` _asbp_gameplay_gamemode))
  (if (`self.IsRandomGoalEnabled`)
    (`/Game/Blueprints/Gameplay/TimerAndGoal/BP_TimerManagerComponent.Register Goal` (`/Game/Blueprints/Gameplay/Gamemode/BP_GameplayGamemode.BP_TimerManagerComponent` _output_get))))

(event `self.Goal Box Collider.OnComponentBeginOverlap`
  (params (OverlappedComponent :type "PrimitiveComponent Object Reference") (OtherActor :type "Actor Object Reference") (OtherComp :type "PrimitiveComponent Object Reference") (OtherBodyIndex :type Integer) (bFromSweep :type Boolean) (SweepResult :type "HitResult Structure (by ref)"))
  ; Goal detects if the player collides with it. From there, it will call the goal collision.
  (bind _asbp_player_character (cast `/Game/Blueprints/Gameplay/Character/BP_PlayerCharacter` OtherActor))
  (bind _output_get (set `self.As BP Player Character` _asbp_player_character))
  (bind (_score_deposited _character) (`/Game/Blueprints/Gameplay/Character/BP_FishingComponent.Deposit Fish` (`/Game/Blueprints/Gameplay/Character/BP_PlayerCharacter.BPC_Fishing` _output_get) (`self.Acceptable Fish`)))
  ;; Passes in the fish point value and player to BP_GoalManagerComponent.
  (`/Game/Blueprints/Gameplay/TimerAndGoal/BP_GoalManagerComponent.Goal Collision` (`/Game/Blueprints/Gameplay/Gamemode/BP_GameplayGamemode.BP_GoalManagerComponent` (`self.As BP Gameplay Gamemode`)) _character _score_deposited))

(event `Change Accptable Fish`
  ; Changes the acceptable fish type. Can be enabled/disabled dependant on "Is Random Goal Enabled". This is enabled when that bool is set to true.
)

(fn `UserConstructionScript`)