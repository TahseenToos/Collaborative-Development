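; Timer manager owned by BP_GameplayGamemode that runs a round's introduction countdown, then its gameplay countdown.
; BeginPlay starts the intro for testing, and its expiry starts the gameplay countdown, which fetches the Goal Manager from the gamemode.
; Each countdown uses a looping one-second timer, printing remaining time as a UI placeholder, then resetting and clearing itself.
; When gameplay time runs out, it calls EndGameplayCountdown on the Goal Manager.
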(event `self.ReceiveBeginPlay`
  ; Introduction Countdown Timer
  ;; Starts the "Start Introduction Countdown" timer for testing purposes.
  (`self.Start Intro Coundown`))

(event `Start Intro Coundown`
  ; Introduction Countdown Timer
  ;; Introduction Countdown Timer, Set Timer.
  (set `self.Current Intro Countdown` (`self.Intro Countdown Length`))
  (bind _returnvalue (`KismetSystemLibrary.K2_SetTimerDelegate` (`|CreateDelegate` :!event `Intro Countdown Iteration`) 1.0 true))
  (set `self.Introduction Countdown Handler` _returnvalue))

(event `Intro Countdown Iteration`
  (bind _current_intro_countdown (`self.Current Intro Countdown`))
  ; Introduction Countdown Timer
  ;; Starts the logic behind the Introduction Countdown timer.
  (if (> (`self.Current Intro Countdown`) 0.0)
    ;; This is where you should change UI display
    (`KismetSystemLibrary.PrintString` (`KismetStringLibrary.Conv_DoubleToString` _current_intro_countdown))
    ;; If Intro Countdown Timer is active, logic.
    (`/Engine/EditorBlueprintResources/StandardMacros.DecrementFloat` _current_intro_countdown)
    (else
      (`self.Start Gameplay Countdown`)
      (`KismetSystemLibrary.PrintString` "START!")
      ;; If Intro Countdown Timer is not active, logic.
      (set `self.Current Intro Countdown` (`self.Intro Countdown Length`))
      (`KismetSystemLibrary.K2_ClearAndInvalidateTimerHandle` (`self.Introduction Countdown Handler`)))))

(event `Start Gameplay Countdown`
  ; Gameplay Countdown Timer
  ;; Gameplay Countdown Timer, Set Timer.
  (set `self.Current Gameplay Countdown` (`self.Gameplay Countdown Length`))
  (bind _returnvalue (`KismetSystemLibrary.K2_SetTimerDelegate` (`|CreateDelegate` :!event `Gameplay Countdown Iteration`) 1.0 true))
  (set `self.Gameplay Countdown Handler` _returnvalue)
  ;; Sets up the reference to Goal Manager
  (bind _asbp_gameplay_gamemode (cast `/Game/Blueprints/Gameplay/BP_GameplayGamemode` (`self.GetOwner`)))
  (set `self.Goal Manager` (`/Game/Blueprints/Gameplay/BP_GameplayGamemode.BP_Goal_Manager` _asbp_gameplay_gamemode)))

(event `Gameplay Countdown Iteration`
  (bind _current_gameplay_countdown (`self.Current Gameplay Countdown`))
  ; Gameplay Countdown Timer
  ;; Starts the logic behind the Gameplay Countdown timer.
  (if (> (`self.Current Gameplay Countdown`) 0.0)
    ;; This is where you should change UI display
    (`KismetSystemLibrary.PrintString` (`KismetStringLibrary.Conv_DoubleToString` _current_gameplay_countdown))
    ;; If Gameplay Countdown Timer is active, logic.
    (`/Engine/EditorBlueprintResources/StandardMacros.DecrementFloat` _current_gameplay_countdown)
    (else
      (`KismetSystemLibrary.PrintString` "ROUND FINISHED!")
      ;; If Gameplay Countdown Timer is not active, logic.
      (`/Game/Blueprints/Gameplay/TimerAndGoal/BP_Goal_Manager.End Gameplay Countdown` (`self.Goal Manager`))
      (set `self.Current Gameplay Countdown` (`self.Gameplay Countdown Length`))
      (`KismetSystemLibrary.K2_ClearAndInvalidateTimerHandle` (`self.Gameplay Countdown Handler`)))))