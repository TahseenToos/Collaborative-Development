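; Timer manager component that runs an introduction countdown from BeginPlay, then the gameplay countdown, using looping one-second timers.
; Event dispatchers broadcast countdown updates and the intro's finish, and the goal manager is notified when gameplay time expires.
; RegisterGoal caches all BP_Goal actors.
; Gameplay time is split into intervals at which the randomised goal list, which only takes the first random-enabled goal, changes its accepted fish.
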(event `Register Goal`
  ; Registers the goal in an array list.
  ;; Assigns all the existing goals into the goal array.
  (bind _outactors (`GameplayStatics.GetAllActorsOfClass` "/Game/Blueprints/Gameplay/TimerAndGoal/BP_Goal.BP_Goal_C"))
  (bind _output_get (set `self.Goal List` _outactors))
  (for _ _output_get
    _))

(event `self.ReceiveBeginPlay`
  ; Introduction Countdown Timer
  ;; Starts the "Start Introduction Countdown" timer for testing purposes.
  (`self.Start Intro Coundown`))

(event `Intro Countdown Iteration`
  (bind _timer_manager_struct_startcountdownlength (break `/Game/Blueprints/Gameplay/Structs/TimerManagerStruct/S_Timer_Manager_Structure` (`self.Timer Manager Struct`)))
  ; Introduction Countdown Timer
  ;; Starts the logic behind the Introduction Countdown timer.
  (`self.On Start Timer Update` (`self.Current Intro Countdown`))
  (if (> (`self.Current Intro Countdown`) 0)
    ;; If Intro Countdown Timer is active, logic.
    (set `self.Current Intro Countdown` (- (`self.Current Intro Countdown`) 1))
    (else
      ;; This is where you should change UI display
      (`self.Start Gameplay Countdown`)
      ;; If Intro Countdown Timer is not active, logic.
      (set `self.Current Intro Countdown` _timer_manager_struct_startcountdownlength)
      (`KismetSystemLibrary.K2_ClearAndInvalidateTimerHandle` (`self.Introduction Countdown Handler`))
      (`self.On Start Timer Finished`))))

(event `Start Intro Coundown`
  (bind (_timer_manager_struct_startcountdownlength _timer_manager_struct_gameplaycountdownlength) (break `/Game/Blueprints/Gameplay/Structs/TimerManagerStruct/S_Timer_Manager_Structure` (`self.Timer Manager Struct`)))
  ; Introduction Countdown Timer
  ;; Introduction Countdown Timer, Set Timer.
  (set `self.Current Intro Countdown` _timer_manager_struct_startcountdownlength)
  (bind _returnvalue (`KismetSystemLibrary.K2_SetTimerDelegate` (`|CreateDelegate` :!event `Intro Countdown Iteration`) 1.0 true false -1.0))
  (set `self.Introduction Countdown Handler` _returnvalue)
  (`self.Calculate Goal Update Intervals` _timer_manager_struct_gameplaycountdownlength))

(event `Update Timer Display`
  (params (`Time (Seconds)` :type Integer))
  ; Updates the time remaining for UI.
  (`self.On Timer Update` `Time (Seconds)`))

(event `Start Gameplay Countdown`
  (bind (_timer_manager_struct_startcountdownlength _timer_manager_struct_gameplaycountdownlength) (break `/Game/Blueprints/Gameplay/Structs/TimerManagerStruct/S_Timer_Manager_Structure` (`self.Timer Manager Struct`)))
  ; Gameplay Countdown Timer
  ;; Gameplay Countdown Timer, Set Timer.
  (set `self.Current Gameplay Countdown` _timer_manager_struct_gameplaycountdownlength)
  (bind _returnvalue (`KismetSystemLibrary.K2_SetTimerDelegate` (`|CreateDelegate` :!event `Gameplay Countdown Iteration`) 1.0 true false -1.0))
  (set `self.Gameplay Countdown Handler` _returnvalue))

(event `Gameplay Countdown Iteration`
  (bind (_timer_manager_struct_startcountdownlength _timer_manager_struct_gameplaycountdownlength) (break `/Game/Blueprints/Gameplay/Structs/TimerManagerStruct/S_Timer_Manager_Structure` (`self.Timer Manager Struct`)))
  (bind _current_gameplay_countdown (`self.Current Gameplay Countdown`))
  ; Gameplay Countdown Timer
  ;; Starts the logic behind the Gameplay Countdown timer.
  (if (>= (`self.Current Gameplay Countdown`) 0)
    ;; This is where you should change UI display
    (`self.Update Timer Display` _current_gameplay_countdown)
    ;; Logic for if the Gameplay Countdown timer is active
    (`self.Check For Goal Update` _current_gameplay_countdown)
    (set `self.Current Gameplay Countdown` (- _current_gameplay_countdown 1))
    (else
      ;; Logic for if the Gameplay Countdown timer is not active
      (`/Game/Blueprints/Gameplay/TimerAndGoal/BP_GoalManagerComponent.End Gameplay Countdown` (`self.Goal Manager`))
      (set `self.Current Gameplay Countdown` _timer_manager_struct_gameplaycountdownlength)
      (`KismetSystemLibrary.K2_ClearAndInvalidateTimerHandle` (`self.Gameplay Countdown Handler`)))))

(event `Calculate Goal Update Intervals`
  (params (`Time (Seconds)` :type Integer))
  (bind _randomised_goal_list (`self.Randomised Goal List`))
  ; Calculates the update interval.
  ;; Runs a check to find if any goals are randomised.
  (for _array_element (`self.Goal List`)
    (if (`/Game/Blueprints/Gameplay/TimerAndGoal/BP_Goal.IsRandomGoalEnabled` _array_element)
      (if (`KismetArrayLibrary.Array_IsEmpty` _randomised_goal_list)
        (`KismetArrayLibrary.Array_Add` _randomised_goal_list _array_element))))
  ;; If any of the goals are randomised, calculate an interval.
  (if (> (`KismetArrayLibrary.Array_Length` (`self.Randomised Goal List`)) 0)
    (set `self.Update Goal Interval` (`KismetMathLibrary.FTrunc` (/ (`KismetMathLibrary.Conv_IntToDouble` `Time (Seconds)`) (`KismetMathLibrary.Conv_IntToDouble` (`self.Goal Randomisation Number`)))))
    (set `self.IsRandomGoalsEnabled` true)))

(event `Check For Goal Update`
  (params (`Time (Seconds)` :type Integer))
  (bind _update_goal_interval (`self.Update Goal Interval`))
  ; Goal Update Check. This updates the goal if the gameplay timer hits a valid interval between goal changes.
  ;; Validates if randomisation is enabled.
  (if (`self.IsRandomGoalsEnabled`)
    ;; Checks if the current timer is a number divisable by the interval value - specifically if it's the last change.
    (if (== (mod `Time (Seconds)` _update_goal_interval) 0)
      ;; Changes the goal's accepted fish for the last time.
      (for _array_element (`self.Randomised Goal List`)
        (`/Game/Blueprints/Gameplay/TimerAndGoal/BP_Goal.Change Accptable Fish` _array_element))
      (else
        ;; Changes the goal's accepted fish if it's on the majority of changes.
        (if (== (`KismetMathLibrary.FTrunc` (`KismetMathLibrary.FMod64` (`KismetMathLibrary.Conv_IntToDouble` `Time (Seconds)`) (`KismetMathLibrary.Conv_IntToDouble` _update_goal_interval))) 0)
          (for _array_element_2 (`self.Randomised Goal List`)
            (`/Game/Blueprints/Gameplay/TimerAndGoal/BP_Goal.Change Accptable Fish` _array_element_2)))))))

(fn `Gamemode Setter`
  (params (Gamemode :type "/Game/Blueprints/Gameplay/Gamemode/BP_GameplayGamemode Object Reference"))
  (set `self.Gamemode` Gamemode))

(fn `Goal Manager Setter`
  (params (`Goal Manager` :type "/Game/Blueprints/Gameplay/TimerAndGoal/BP_GoalManagerComponent Object Reference"))
  (set `self.Goal Manager` `Goal Manager`))