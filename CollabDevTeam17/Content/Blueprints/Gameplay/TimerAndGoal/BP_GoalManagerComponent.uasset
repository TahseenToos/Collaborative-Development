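; Goal manager component that is an unfinished scaffold for scoring caught fish when a player reaches a goal.
; GoalCollision prints the collision, then IncreasePlayerScore loops over the player's caught fish and searches PlayerMap for that player's entry.
; The score write is missing, with the point addition left unconnected; BeginPlay only zeroes CurrentPlayerScore.
; The countdown-end winner event and Players function are empty, and the winner and score announcements never run.
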(event `self.ReceiveBeginPlay`
  ; Intended to set all player scores to zero.
  (set `self.Current Player Score` 0.0))

(event `/Game/Blueprints/Gameplay/Interface/BPI_Goal_Interface.Goal Collision`
  (params (Player :type "/Game/Blueprints/Gameplay/Character/BP_PlayerCharacter Object Reference") (Goal :type "/Game/Blueprints/Gameplay/TimerAndGoal/BP_Goal Object Reference"))
  ; Goal collision handler. Triggers the "Increases player score" section.
  ;; When a goal is collided with.
  ;; Intended to get: the goal, the player and the fish the player has.
  (`KismetSystemLibrary.PrintString` (`KismetStringLibrary.Concat_StrStr` (`KismetSystemLibrary.GetDisplayName` Player) " collided with " (`KismetSystemLibrary.GetDisplayName` Goal)))
  ;; Trigger the increase of the player score here.
  (`self.Increase Player Score` Player))

(event `Increase Player Score`
  (params (Player :type "/Game/Blueprints/Gameplay/Character/BP_PlayerCharacter Object Reference"))
  ; Increases player score.
  ;; When the player score event is triggered
  ;; Sets the player key. Also gets the point value of all caught fish.
  (set `self.Player` Player)
  (for _array_element (`/Game/Blueprints/Gameplay/Character/BP_FishingComponent.Caught Fish Getter` (`/Game/Blueprints/Gameplay/Character/BP_PlayerCharacter.BPC_Fishing` Player))
    ;; Set the correct player's map score to the new point value.
    (bind _keypin (`|MapForEach` (`self.Player Map`))
      (:`then`
        (if (== _keypin (`self.Player`))
          _)))))

(event `End Gameplay Countdown`
  ; This section is to find the winner. Multiplayer required to do this.
)

(fn `Players`
  (params (`Player 1` :type Boolean)))