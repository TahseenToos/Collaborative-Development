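; BP_FishingSpot is a fishing spot actor that can be switched between active and inactive states.
; Activation and deactivation events set the IsActive flag and swap the mesh material between an active highlight and the default cached on BeginPlay.
; A capsule overlap keeps a list of nearby actors as PlayersNearFishingSpot, without filtering by type.
; The Fishing event only prints a debug message while the spot is active.
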(event `self.ReceiveBeginPlay`
  ; Sets default material on BeginPlay
  (set `self.Default Mat` (`PrimitiveComponent.GetMaterial` (`self.FishingSpotMesh`) 0)))

(event `self.Capsule.OnComponentBeginOverlap`
  (params (OverlappedComponent :type "PrimitiveComponent Object Reference") (OtherActor :type "Actor Object Reference") (OtherComp :type "PrimitiveComponent Object Reference") (OtherBodyIndex :type Integer) (bFromSweep :type Boolean) (SweepResult :type "HitResult Structure (by ref)"))
  ; Sorts reference to all players close to it
  (`KismetArrayLibrary.Array_AddUnique` (`self.PlayersNearFishingSpot`) OtherActor))

(event `self.Capsule.OnComponentEndOverlap`
  (params (OverlappedComponent :type "PrimitiveComponent Object Reference") (OtherActor :type "Actor Object Reference") (OtherComp :type "PrimitiveComponent Object Reference") (OtherBodyIndex :type Integer))
  ; Sorts reference to all players close to it
  (`KismetArrayLibrary.Array_RemoveItem` (`self.PlayersNearFishingSpot`) OtherActor))

(event `/Game/Blueprints/Gameplay/I_Fishing.Fishing`
  (params (PlayerFishing :type "Actor Object Reference"))
  ; Activates fishing in the player
  (if (`self.Is Active`)
    (`KismetSystemLibrary.PrintString` "actively fishing")))

(event `Activate Fishing Spot`
  ; Activates spot to be fishable
  (set `self.Is Active` true)
  (`PrimitiveComponent.SetMaterial` (`self.FishingSpotMesh`) 0 "/Game/Blueprints/Material/M_ActivateFishingSpot.M_ActivateFishingSpot"))

(event `Deactivate Fishing Spot`
  ; Deactivates spot to no longer be fishable
  (set `self.Is Active` false)
  (`PrimitiveComponent.SetMaterial` (`self.FishingSpotMesh`) 0 (`self.Default Mat`)))

(fn `UserConstructionScript`)