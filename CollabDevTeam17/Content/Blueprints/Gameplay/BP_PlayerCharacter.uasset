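; Player character that moves relative to a shared local multiplayer camera and can start a fishing minigame at fishing spots.
; Enhanced Input drives movement, controller look and fishing, which passes the current spot to TestFishingComp.
; Capsule overlaps store a BP_FishingSpot reference and clear it on any overlap end.
; MoveActor lazily finds the camera and blocks input away from it beyond per-axis range limits, measured along the camera's right and up vectors.
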(event `EnhancedInput|/Game/Inputs/PlayerMovement/Keybinds/IA_Move`
  (params (ActionValue :type "Vector2D Structure") (ElapsedSeconds :type "Float (double-precision)") (TriggeredSeconds :type "Float (double-precision)") (InputAction :type "InputAction Object Reference" :default "/Game/Inputs/PlayerMovement/Keybinds/IA_Move.IA_Move"))
  ; Allows player movement to be controlled
  (:`Triggered`
    (`self.Move Actor` ActionValue_X ActionValue_Y)))

(event `EnhancedInput|/Game/Inputs/PlayerMovement/Keybinds/IA_Look`
  (params (ActionValue :type "Vector2D Structure") (ElapsedSeconds :type "Float (double-precision)") (TriggeredSeconds :type "Float (double-precision)") (InputAction :type "InputAction Object Reference" :default "/Game/Inputs/PlayerMovement/Keybinds/IA_Look.IA_Look"))
  ; Allows player looking to be controlled
  (:`Triggered`
    (`self.AddControllerYawInput` ActionValue_X)
    (`self.AddControllerPitchInput` ActionValue_Y)))

(event `EnhancedInput|/Game/Inputs/PlayerMovement/Keybinds/IA_Fish`
  (params (ActionValue :type Boolean) (ElapsedSeconds :type "Float (double-precision)") (TriggeredSeconds :type "Float (double-precision)") (InputAction :type "InputAction Object Reference" :default "/Game/Inputs/PlayerMovement/Keybinds/IA_Fish.IA_Fish"))
  ; Activates fishing when button is pressed and near fishing spot
  (:`Started`
    (`/Game/Blueprints/Gameplay/BPC_Fishing.TriggerFishingMinigame` (`self.TestFishingComp`) (`self.Fishing Spot`))))

(event `self.CapsuleComponent.OnComponentBeginOverlap`
  (params (OverlappedComponent :type "PrimitiveComponent Object Reference") (OtherActor :type "Actor Object Reference") (OtherComp :type "PrimitiveComponent Object Reference") (OtherBodyIndex :type Integer) (bFromSweep :type Boolean) (SweepResult :type "HitResult Structure (by ref)"))
  ; Grabs fishing spot ref if close enough
  (if (== (`GameplayStatics.GetObjectClass` OtherActor) "/Game/Blueprints/Gameplay/BP_FishingSpot.BP_FishingSpot_C")
    (set `self.Fishing Spot` OtherActor)))

(event `self.CapsuleComponent.OnComponentEndOverlap`
  (params (OverlappedComponent :type "PrimitiveComponent Object Reference") (OtherActor :type "Actor Object Reference") (OtherComp :type "PrimitiveComponent Object Reference") (OtherBodyIndex :type Integer))
  ; Removes fishing spot if too far
  (set `self.Fishing Spot` (`self.Empty Ref`)))

(fn `Move Actor`
  (params (`X Axis` :type "Float (double-precision)") (`Y Axis` :type "Float (double-precision)"))
  (bind _local_multiplayer_camera (`self.Local Multiplayer Camera`))
  (bind _local_multiplayer_camera_2 (`self.Local Multiplayer Camera`))
  (bind (_returnvalue_roll _returnvalue_pitch _returnvalue_yaw) (`KismetMathLibrary.BreakRotator` (`SceneComponent.K2_GetComponentRotation` (`/Game/Blueprints/Camera/BP_LocalMultiplayerCamera.Camera` (`self.Local Multiplayer Camera`)))))
  (bind (_returnvalue_roll_2 _returnvalue_pitch_2 _returnvalue_yaw_2) (`KismetMathLibrary.BreakRotator` (`SceneComponent.K2_GetComponentRotation` (`/Game/Blueprints/Camera/BP_LocalMultiplayerCamera.Camera` (`self.Local Multiplayer Camera`)))))
  (bind _returnvalue (`KismetMathLibrary.Dot_VectorVector` (- (`self.K2_GetActorLocation` _local_multiplayer_camera_2) (`self.K2_GetActorLocation`)) (`KismetMathLibrary.GetUpVector` (`SceneComponent.K2_GetComponentRotation` (`/Game/Blueprints/Camera/BP_LocalMultiplayerCamera.Camera` _local_multiplayer_camera_2)))))
  (bind _returnvalue_2 (`KismetMathLibrary.Dot_VectorVector` (- (`self.K2_GetActorLocation` _local_multiplayer_camera) (`self.K2_GetActorLocation`)) (`KismetMathLibrary.GetRightVector` (`SceneComponent.K2_GetComponentRotation` (`/Game/Blueprints/Camera/BP_LocalMultiplayerCamera.Camera` _local_multiplayer_camera)))))
  (`|ExecutionSequence`
    (:`then_0`
      (`self.Local Multiplayer Camera`
        (:`then`)
        (:`else`
          (bind _returnvalue_3 (`GameplayStatics.GetActorOfClass` "/Game/Blueprints/Camera/BP_LocalMultiplayerCamera.BP_LocalMultiplayerCamera_C"))
          (set `self.Local Multiplayer Camera` _returnvalue_3))))
    (:`then_1`
      (`self.AddMovementInput` (`KismetMathLibrary.GetRightVector` (`KismetMathLibrary.MakeRotator` _returnvalue_roll 0.0 _returnvalue_yaw)) (`KismetMathLibrary.SelectFloat` (`local.X Axis`) 0.0 (or (< (`KismetMathLibrary.Abs` _returnvalue_2) (`self.Max X Movement Range From Camera`)) (and (> _returnvalue_2 0.0) (> (`local.X Axis`) 0.0)) (and (< _returnvalue_2 0.0) (< (`local.X Axis`) 0.0)))))
      (`self.AddMovementInput` (`KismetMathLibrary.GetForwardVector` (`KismetMathLibrary.MakeRotator` 0.0 0.0 _returnvalue_yaw_2)) (`KismetMathLibrary.SelectFloat` (`local.Y Axis`) 0.0 (or (< (`KismetMathLibrary.Abs` _returnvalue) (`self.Max Y Movement Range From Camera`)) (and (> _returnvalue 0.0) (> (`local.Y Axis`) 0.0)) (and (< _returnvalue 0.0) (< (`local.Y Axis`) 0.0))))))))

(fn `UserConstructionScript`)