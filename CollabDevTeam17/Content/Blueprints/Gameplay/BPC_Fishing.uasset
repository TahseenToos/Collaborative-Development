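; Player fishing component that starts the fishing minigame, runs its QTE UI and stores caught fish.
; It messages fishing spots through an interface, then creates a UI_FishingDisplay widget for the owning controller from the supplied fish info.
; The IA_FishQTE input is forwarded to that widget by interface message, and successful catches are appended to CaughtFish.
; A debug key prints the names of caught fish.
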(event Custom|Start%20Fishing%20QTE
  (params (Fish%20Info :type S%20Fish%20Stats%20Structure))
  (bind _owning_controller (Variables|Default|GetOwning%20Controller))
  (Variables|Default|SetCaught%20Fish%20Info (.CaughtFishInfo (Utilities|Struct|BreakS_FishStats Fish%20Info)))
  (Utilities|IsValid _owning_controller
    (:Is%20Valid
      (bind _returnvalue (UserInterface|CreateWidget "/Game/UI/UI_FishingDisplay.UI_FishingDisplay_C" _owning_controller Fish%20Info))
      (bind _output_get (Variables|Default|SetFishingQTEUI _returnvalue))
      (UserInterface|Viewport|AddtoViewport _output_get 0))))

(event Custom|TriggerFishingMinigame
  (params (FishingSpot :type Actor%20Object%20Reference))
  ;[0.15 0.15 0.15 0.5] Calls interface event for fishing spot
  (Class|IFishing|Fishing(Message) FishingSpot self))

(event Custom|Fishing%20Successful
  (params (NewParam :type S%20Caught%20Fish%20Structure))
  (Utilities|Array|Add (Variables|Default|GetCaught%20Fish) NewParam)
  (Development|PrintString "added fish"))

(event Input|EnhancedActionEvents|EnhancedInputActionIA_FishQTE
  (params (ActionValue :type Boolean) (ElapsedSeconds :type Float%20%28double-precision%29) (TriggeredSeconds :type Float%20%28double-precision%29) (InputAction :type Input%20Action%20Object%20Reference :default "/Game/Inputs/PlayerMovement/Keybinds/IA_FishQTE.IA_FishQTE"))
  (:Started
    (Class|IFishing|FishingQTE(Message) (Variables|Default|GetFishingQTEUI) self)))

(event EventBeginPlay)

(event EventTick
  (params (DeltaSeconds :type Float%20%28single-precision%29)))

(event Input|KeyboardEvents|DebugKeyM
  (params (Key :type Key%20Structure :default "None") (ActionValue :type Input%20Action%20Value%20Structure))
  (:Pressed
    (for _array_element (Variables|Default|GetCaught%20Fish)
      (Development|PrintString (Utilities|String|ToString(Name) (.FishName (Utilities|Struct|BreakS_CaughtFish _array_element)))))))

(fn OwningControllerSetter
  (params (Controller :type Player%20Controller%20Object%20Reference))
  (Variables|Default|SetOwning%20Controller Controller))