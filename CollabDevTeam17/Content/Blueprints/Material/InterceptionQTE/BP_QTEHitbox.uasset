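; BP_QTEHitbox is a trigger actor that starts a fish-stealing quick-time event when the player pawn overlaps it.
; On overlap, if no event is active, it creates WBP_InterceptionQTE with its inputs and reaction time, shows it on a widget component and matches its size to the draw size.
; The widget's finished event clears the display and active flag, then prints success or failure as a placeholder for the fish-taking logic.
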(event `self.ReceiveActorBeginOverlap`
  (params (OtherActor :type "Actor Object Reference"))
  (bind (_returnvalue_x _returnvalue_y) (`KismetMathLibrary.BreakVector2D` (`WidgetComponent.GetDrawSize` (`self.Widget`))))
  (bind _sb_qte (`/Game/Blueprints/InterceptionQTE/WBP_InterceptionQTE.SB_QTE` (`self.QTEAlt`)))
  ; Making sure the character is the one overlapping, and making sure another QTE is not already active. Then creating the widget
  (if (and (== OtherActor (`GameplayStatics.GetPlayerPawn` 0)) (not (`self.IsActive?`)))
    (bind _returnvalue (`|CreateWidget` "/Game/Blueprints/InterceptionQTE/WBP_InterceptionQTE.WBP_InterceptionQTE_C" null (`self.QTE Inputs`) (`self.Time to React`)))
    (`WidgetComponent.SetWidget` (`self.Widget`) _returnvalue)
    (bind _output_get (set `self.QTEAlt` _returnvalue))
    (add `/Game/Blueprints/InterceptionQTE/WBP_InterceptionQTE.E_FinishedQTE` _output_get (delegate `FinishedQTE`))
    ; Making sure Widget size is correct
    (set `self.IsActive?` true)
    (`SizeBox.SetHeightOverride` _sb_qte _returnvalue_y)
    (`SizeBox.SetWidthOverride` _sb_qte _returnvalue_x)))

(event `FinishedQTE`
  (params (Success :type Boolean))
  ; QTE Finished event, either Failed or Succsessful
  (set `self.IsActive?` false)
  ;; To be replaced with taking fish or failing to take fish. Widget sets are to remove the widget from the world. Unbind node to be removed if it causes issues
  (clear `/Game/Blueprints/InterceptionQTE/WBP_InterceptionQTE.E_FinishedQTE` (`self.QTEAlt`))
  (`WidgetComponent.SetWidget` (`self.Widget`) null)
  (set `self.QTE` null)
  (if Success
    (`KismetSystemLibrary.PrintString` "FISH STOLEN" true true (struct :`G` 1.0 :`B` 0.096259 :`A` 1.0))
    (else
      (`KismetSystemLibrary.PrintString` "FAILED TO STEAL" true true (struct :`R` 1.0 :`B` 0.011045 :`A` 1.0)))))

(fn `UserConstructionScript`)